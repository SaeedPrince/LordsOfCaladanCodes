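; Fortress building Blueprint that configures its parent class as an item stack and person generator with civilian and military capacity limits.
; The construction script sets those flags and limits after the parent's script.
; On BeginPlay, the authority tints the Border green through a dynamic material instance and scales it, with the second scale call overriding the first.
; Disconnected nodes hold unused Hilltop-specific item stack placement and a server activity start.
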(event EventBeginPlay
  (bind _border (Variables|Default|GetBorder))
  (|CallParentFunction)
  (Networking|SwitchHasAuthority
    (:Authority
      (bind _returnvalue (Rendering|Material|CreateDynamicMaterialInstance _border 0 0 :!class /Script/Engine.PrimitiveComponent))
      (Rendering|Material|SetVectorParameterValue _returnvalue "GlassColor" (CallFunction|GetColorbyString "Green") :!class /Script/Engine.MaterialInstanceDynamic)
      (Transformation|SetWorldScale3D _border "600.000000,600.000000,100.000000")
      (Transformation|SetWorldScale3D (Variables|Default|GetBorder) "100.000000,100.000000,50.000000"))))

(fn ConstructionScript
  (|CallParentFunction)
  (Variables|Default|SetIsStack true)
  (Variables|Default|SetMaxItemCount 32)
  (Variables|Default|SetIsPersonGenerator true)
  (Variables|Default|SetGenerationCount 8)
  (Variables|Default|SetMaxCivil 24)
  (Variables|Default|SetMaxMilitary 24))