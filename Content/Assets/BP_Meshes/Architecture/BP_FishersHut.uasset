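; BP_FishersHut is a Blueprint for a fisher's hut building that produces an item using workers.
; Its construction script runs the parent's, then marks it productive with a single worker slot, a production period offset by a few hours from the default time, an output item index and an inner border radius.
; BeginPlay only calls the parent, so the production behavior itself lives in the parent class.
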(event EventBeginPlay
  (|CallParentFunction))

(fn ConstructionScript
  (|CallParentFunction)
  (Variables|Default|SetIsProductive true)
  (Variables|Default|SetMaxWorker 1)
  (Variables|Default|SetProductionPeriod (+ (Variables|Default|GetDefaultTime) (Math|Timespan|MakeTimespan 0 3)))
  (Variables|Default|SetProduction1ItemIndex 8)
  (Variables|Default|SetInnerBorderRadius 35.0))