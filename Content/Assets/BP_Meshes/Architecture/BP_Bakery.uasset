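; BP_Bakery is a productive building that consumes two item types and produces two others.
; Its construction script runs the parent's script, then configures inherited production variables: single-worker capacity, a production period in hours, and item indices for both inputs and both outputs.
; The file holds only this configuration, with no production logic of its own.
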(fn ConstructionScript
  (|CallParentFunction)
  (Variables|Default|SetIsProductive true)
  (Variables|Default|SetMaxWorker 1)
  (Variables|Default|SetProductionPeriod (+ (Variables|Default|GetDefaultTime) (Math|Timespan|MakeTimespan 0 4)))
  (Variables|Default|SetProduction1ItemIndex 6)
  (Variables|Default|SetIsProducing2 true)
  (Variables|Default|SetProduction2ItemIndex 7)
  (Variables|Default|SetIsConsumer true)
  (Variables|Default|SetConsume1ItemIndex 4)
  (Variables|Default|SetIsConsume2 true)
  (Variables|Default|SetConsume2ItemIndex 5))