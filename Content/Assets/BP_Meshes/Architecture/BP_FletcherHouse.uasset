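; Fletcher house building Blueprint that configures a worker-staffed production building which turns consumed items into produced goods.
; Its construction script runs the parent script, then sets inherited production and consumption fields for two output items and two input items, referenced by index.
; It also caps the worker count and sets the production period as an hours offset from a default time.
; The file holds only this configuration, with no production logic of its own.
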(fn ConstructionScript
  (|CallParentFunction)
  (Variables|Default|SetIsProductive true)
  (Variables|Default|SetMaxWorker 2)
  (Variables|Default|SetProductionPeriod (+ (Variables|Default|GetDefaultTime) (Math|Timespan|MakeTimespan 0 3)))
  (Variables|Default|SetProduction1ItemIndex 18)
  (Variables|Default|SetIsProducing2 true)
  (Variables|Default|SetProduction2ItemIndex 27)
  (Variables|Default|SetIsConsumer true)
  (Variables|Default|SetConsume1ItemIndex 0)
  (Variables|Default|SetIsConsume2 true)
  (Variables|Default|SetConsume2ItemIndex 30))