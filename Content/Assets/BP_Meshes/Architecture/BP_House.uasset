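; Building Blueprint for an economy game, configured by flags as producer, consumer and/or stack (storage hub), with resident civilian and military counts.
; Arriving civilians start per-worker looping timers, bound by function name, that consume inputs and spawn BP_Items.
; Producers and consumers queue pickup and item demands at their nearest stack.
; The stack's timer assigns the nearest free "Career" (carrier), serving pickups before demands.
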(event Custom|ServerReceiveItemSentReport
  (params (ItemIndex :type Integer))
  ;[1 1 0] Happens in consumer when stack sends item
  (bind _returnvalue (Utilities|MacReceiveItemSentReport (Variables|Consume|GetConsume1ItemIndex) (Variables|Demand|GetDemand1Sent) (Variables|Demand|GetDemand1OnTheWay) ItemIndex))
  (if (not _returnvalue)
    (Utilities|MacReceiveItemSentReport (Variables|Consume|GetConsume2ItemIndex) (Variables|Demand|GetDemand2Sent) (Variables|Demand|GetDemand2OnTheWay) ItemIndex)))

(event Custom|ServerReceiveItemDemand
  (params (Demand :type Struct%20Demand%20Structure))
  ;[1 1 0] Happens in stack when receive item demand or pickup demand after production
  (Utilities|Array|Add (Variables|Queue|GetDemandQueue) Demand))

(event Custom|ServerPersonArrivedHome
  (params (PersonType :type Integer) (PersonIndex :type Integer))
  ;[1 1 0] Happens in any building which person arrives
  (switch int PersonType
    (:0
      (Variables|Population|SetCurrentCivilian (+ (Variables|Population|GetCurrentCivilian) 1))
      (if (Variables|Data|GetIsProductive)
        (Utilities|MacStartProduction PersonIndex)
        (if (and (Variables|Data|GetIsConsumer) (not (Utilities|Time|IsValidTimerHandle (Variables|Demand|GetTimerDemand))))
          (Utilities|MacStartItemDemand)))
      (if (and (Variables|Data|GetIsStack) (not (Utilities|Time|IsValidTimerHandle (Variables|Stack|GetTimerStack))))
        (Utilities|MacStartStackActivity)))
    (:1
      (Variables|Population|SetCurrentMilitary (+ (Variables|Population|GetCurrentMilitary) 1)))))

(event Custom|ServerItemSent
  (params (Item :type BP%20Item%20Object%20Reference))
  ;[1 1 0] Happens in producer when career picks up the item
  (Utilities|Array|RemoveItem (Variables|Item|GetAvailableItems) Item))

(event Custom|ServerItemReceived
  (params (Item :type BP%20Item%20Object%20Reference))
  ;[1 1 0] Happens in consumer when receives demanded item
  (Utilities|Array|Add (Variables|Item|GetAvailableItems) Item))

(event Custom|ServerPersonLeftHome
  (params (PersonType :type Integer) (PersonIndex :type Integer))
  ;[1 1 0] Happens in any building which person leaves
  (switch int PersonType
    (:0
      (Variables|Population|SetCurrentCivilian (- (Variables|Population|GetCurrentCivilian) 1))
      (if (Variables|Data|GetIsProductive)
        (Utilities|MacStopProduction PersonIndex true))
      (if (== (Variables|Population|GetCurrentCivilian) 0)
        (if (Variables|Data|GetIsConsumer)
          (Utilities|MacStopItemDemand))
        (if (Variables|Data|GetIsStack)
          (Utilities|MacStopStackActivity))))
    (:1
      (Variables|Population|SetCurrentMilitary (- (Variables|Population|GetCurrentMilitary) 1)))))

(event Custom|ServerStartActivity
  ;[1 1 0] Assign Stack
  (if (Variables|Data|GetIsProductive)
    (Utilities|MacAssignStack))
  (if (and (Variables|Data|GetIsStack) (not (Utilities|Time|IsValidTimerHandle (Variables|Stack|GetTimerStack))))
    (Utilities|MacStartStackActivity)))

(event Custom|ServerReceivePickupDemand
  (params (Item :type Struct%20Pickup%20Structure))
  ;[1 1 0] Happens in stack when receive item demand or pickup demand after production
  (Utilities|IsValid (.Item (Utilities|Struct|BreakStructPickup Item))
    (:Is%20Valid
      (Development|PrintString "Item pickup demand received. Added to queue." true true "(R=0.000000,G=1.000000,B=0.000000,A=1.000000)" 1e+01)
      (Utilities|Array|Add (Variables|Queue|GetPickupQueue) Item))
    (:Is%20Not%20Valid
      (Development|PrintString "Item pickup demand invalid" true true "(R=1.000000,G=0.000000,B=0.000000,A=1.000000)" 1e+01))))

(event EventBeginPlay
  ;[1 1 0] Begin play
  (Collision|SetCollisionObjectType (Variables|Default|GetHouseMesh) (Variables|SpawnData|GetCollisionObjectType)))

(fn ConstructionScript)

(fn Produce0
  (Utilities|MacProductionCycle))

(fn Produce
  (params (Number :type Integer))
  (bind _productiontime (Variables|Time|GetProductionTime))
  (bind _productionperiod (Variables|Product|GetProductionPeriod))
  (bind _output (Utilities|Array|Get(acopy) _productiontime Number))
  (bind _returnvalue (Class|LordsOfCaladanFunctionLibrary|AddOneScaledSecond _output))
  (bind _returnvalue_2 (>= _returnvalue _productionperiod))
  (if _returnvalue_2
    (LocalVariables|SetOutTime (Variables|DefaultValue|GetDefaultTime))
    (else
      (LocalVariables|SetOutTime _returnvalue)))
  (return _returnvalue_2 (LocalVariables|GetOutTime)))

(fn Produce1
  (Utilities|MacProductionCycle 1))

(fn Produce2
  (Utilities|MacProductionCycle 2))

(fn Produce3
  (Utilities|MacProductionCycle 3))

(fn Produce4
  (Utilities|MacProductionCycle 4))

(fn Demand
  (bind _demandmax (Variables|Demand|GetDemandMax))
  (if (< (+ (Variables|Demand|GetDemand1Sent) (Variables|Demand|GetDemand1OnTheWay) (Variables|Consume|GetConsume1Available)) _demandmax)
    (Utilities|MacDemand (Variables|Consume|GetConsume1ItemIndex))
    (Variables|Demand|SetDemand1Sent (+ (Variables|Demand|GetDemand1Sent) 1)))
  (if (Variables|Data|GetIsUsingConsume2)
    (if (< (+ (Variables|Demand|GetDemand2Sent) (Variables|Demand|GetDemand2OnTheWay) (Variables|Consume|GetConsume2Available)) _demandmax)
      (Utilities|MacDemand (Variables|Consume|GetConsume2ItemIndex))
      (Variables|Demand|SetDemand2Sent (+ (Variables|Demand|GetDemand2Sent) 1)))))

(fn StackActivity
  (bind _self self)
  (bind _demandqueue (Variables|Queue|GetDemandQueue))
  (bind _pickupqueue (Variables|Queue|GetPickupQueue))
  (bind _output (Utilities|Array|Get(acopy) _pickupqueue))
  (bind _output_2 (Utilities|Array|Get(acopy) _demandqueue))
  (bind _returnvalue (Utilities|MacBuildingItemPlace _self))
  (bind (_building _item) (Utilities|Struct|BreakStructPickup _output))
  (bind (_building_2 _itemindex) (Utilities|Struct|BreakStructDemand _output_2))
  (bind _returnvalue_2 (CallFunction|FindNearestCareer _returnvalue))
  (bind (_available _item_2) (CallFunction|ItemAvailable _itemindex))
  (bind _returnvalue_3 (Utilities|MacBuildingItemPlace _building))
  (bind _returnvalue_4 (CallFunction|FindNearestCareer _returnvalue_3))
  (if (CallFunction|CareerAvailable)
    (if (> (Utilities|Array|Length _pickupqueue) 0)
      (Utilities|IsValid _item
        (:Is%20Valid
          (Development|PrintString "Item valid. Pickup job started." true true "(R=0.000000,G=1.000000,B=0.000000,A=1.000000)" 1e+01)
          (Variables|/Game/Blueprints/Controllers/AIController_Game.AIController_Game_C|SetCarry _returnvalue_4 (Utilities|Struct|MakeStructCarry _building (CallFunction|FindBestDemand (Variables|/Game/Assets/BP_Meshes/Item/BP_Item.BP_Item_C|GetIndex _item)) _item))
          (Utilities|MacSetCareerUnavailable _returnvalue_4)
          (Utilities|Array|RemoveIndex _pickupqueue))
        (:Is%20Not%20Valid
          (Development|PrintString "Item not valid." true true "(R=1.000000,G=0.000000,B=0.000000,A=1.000000)" 1e+01)))
      (elif (> (Utilities|Array|Length _demandqueue) 0)
        (if _available
          (Variables|/Game/Blueprints/Controllers/AIController_Game.AIController_Game_C|SetCarry _returnvalue_2 (Utilities|Struct|MakeStructCarry _self _building_2 _item_2))
          (Utilities|MacSetCareerUnavailable _returnvalue_2)
          (Utilities|Array|RemoveIndex _demandqueue)
          (CallFunction|ServerReceiveItemSentReport _building_2 _itemindex))))))

(fn CareerAvailable
  (bind _array_element (Utilities|Array|ForEachLoopwithBreak (Variables|Queue|GetCareerQueue) :!label _label)
    (:LoopBody
      (if (not (Variables|/Game/Blueprints/Controllers/AIController_Game.AIController_Game_C|GetHasCarry _array_element))
        (LocalVariables|SetOutBool true)
        (goto _label Break)))
    (:Completed
      (return (LocalVariables|GetOutBool)))))

(fn FindBestDemand
  (params (ItemIndex :type Integer))
  (for _array_element (Utilities|Struct|BreakStructPlayer (Variables|/Game/Blueprints/Controllers/PlayerController_Game.PlayerController_Game_C|GetPlayerData (Utilities|Array|Get(acopy) (Variables|/Game/Blueprints/GameModes/GameMode_Game.GameMode_Game_C|GetPlayerControllers (Variables|GameObjects|GetGameModeRef)) (Variables|SpawnData|GetPlayerIndex))))
    (if (and (== (Variables|BP_House_C|GetConsume1ItemIndex (Utilities|Struct|BreakStructBuilding _array_element)) ItemIndex) (> (Variables|BP_House_C|GetDemand1Sent (Utilities|Struct|BreakStructBuilding _array_element)) 0))
      (if (== (LocalVariables|GetOutBuilding) 0)
        (LocalVariables|SetOutBuilding (Utilities|Struct|BreakStructBuilding _array_element) :!label _label)
        (elif (< (Utilities|MacBuildingtoBuildingDestination (Utilities|Struct|BreakStructBuilding _array_element)) (Utilities|MacBuildingtoBuildingDestination (LocalVariables|GetOutBuilding)))
          (goto _label)))))
  (if (== (LocalVariables|GetOutBuilding) 0)
    (LocalVariables|SetOutBuilding self))
  (return (LocalVariables|GetOutBuilding)))

(fn FindNearestCareer
  (params (Location :type Vector))
  (for _array_element (Variables|Queue|GetCareerQueue)
    (if (not (Variables|/Game/Blueprints/Controllers/AIController_Game.AIController_Game_C|GetHasCarry _array_element))
      (if (== (LocalVariables|GetOutCareer) 0)
        (LocalVariables|SetOutCareer _array_element :!label _label)
        (elif (< (Utilities|MacActortoLocationDestination Location (Pawn|GetControlledPawn _array_element)) (Utilities|MacActortoLocationDestination Location (Pawn|GetControlledPawn (LocalVariables|GetOutCareer))))
          (goto _label)))))
  (return (LocalVariables|GetOutCareer)))

(fn ItemAvailable
  (params (ItemIndex :type Integer))
  (bind (_array_element _array_index) (Utilities|Array|ForEachLoopwithBreak (Variables|Item|GetAvailableItems) :!label _label)
    (:LoopBody
      (if (and (not (Variables|/Game/Assets/BP_Meshes/Item/BP_Item.BP_Item_C|GetAssignedToCarry _array_element)) (== _array_index ItemIndex))
        (LocalVariables|SetOutBool true)
        (LocalVariables|SetOutItem _array_element)
        (Variables|/Game/Assets/BP_Meshes/Item/BP_Item.BP_Item_C|SetAssignedToCarry _array_element true)
        (goto _label Break)))
    (:Completed
      (return (LocalVariables|GetOutBool) (LocalVariables|GetOutItem)))))

(fn SpawnItem
  (bind _returnvalue (Game|SpawnActorfromClass "/Game/Assets/BP_Meshes/Item/BP_Item.BP_Item_C" (Math|Transform|MakeTransform (Transformation|GetWorldLocation (Variables|Default|GetItemPlace))) "AlwaysSpawn" 0 (Variables|Product|GetProductionItemIndex) 0))
  (Utilities|IsValid _returnvalue
    (:Is%20Valid
      (Development|PrintString "Item produced and spawned" true true "(R=0.000000,G=1.000000,B=0.000000,A=1.000000)" 1e+01)
      (Utilities|Array|Add (Variables|Item|GetAvailableItems) _returnvalue)
      (LocalVariables|SetOutBool true))
    (:Is%20Not%20Valid
      (Development|PrintString "Item produced, but not  spawned" true true "(R=1.000000,G=0.000000,B=0.000000,A=1.000000)" 1e+01)
      (LocalVariables|SetOutBool false)))
  (return (LocalVariables|GetOutBool) _returnvalue))

(fn GetItemCount
  (params (ItemIndex :type Integer))
  (for _array_element (Variables|Item|GetAvailableItems)
    (if (== (Variables|/Game/Assets/BP_Meshes/Item/BP_Item.BP_Item_C|GetIndex _array_element) ItemIndex)
      (LocalVariables|SetOutInteger (+ (LocalVariables|GetOutInteger) 1))))
  (return (LocalVariables|GetOutInteger)))