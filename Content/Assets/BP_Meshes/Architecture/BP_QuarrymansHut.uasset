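; BP_QuarrymansHut is a building Blueprint for a quarryman's hut, configured as an owned, productive structure with worker slots.
; Its construction script calls the parent, then sets inherited properties for worker capacity, production period, produced item index, inner border radius and mesh size.
; BeginPlay only forwards to the parent, so this child adds configuration and no runtime logic of its own.
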(event EventBeginPlay
  (|CallParentFunction))

(fn ConstructionScript
  (|CallParentFunction)
  (Variables|Default|SetIsProductive true)
  (Variables|Default|SetMaxWorker 2)
  (Variables|Default|SetProductionPeriod (+ (Variables|Default|GetDefaultTime) (Math|Timespan|MakeTimespan 0 4)))
  (Variables|Default|SetProduction1ItemIndex 1)
  (Variables|Default|SetInnerBorderRadius 2.5e+03)
  (Variables|Default|SetMeshSize 1e+02)
  (Variables|Default|SetHasOwner true))