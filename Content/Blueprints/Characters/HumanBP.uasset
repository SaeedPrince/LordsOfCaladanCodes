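; Networked human player character with modular appearance, movement, bow holstering and switchable FPS, RTS and TPS cameras.
; Multicast events swap body, clothing and hair meshes, tinting them through dynamic material instances, with parts following the main mesh via master pose.
; Turning, walk/run speed and ranged weapon changes relay from server to multicast events.
; Camera switches toggle owner visibility between mesh sets; melee and shield events are empty stubs.
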(event Custom|SetPlayerColorForEveryone
  (params (PlayerColor :type Linear%20Color%20Structure))
  ;[1 1 0] Player color shows on sphere top of head
  (bind _returnvalue (Rendering|Material|CreateDynamicMaterialInstance (Variables|Default|GetPlayerColorSphere) 0 0 :!class /Script/Engine.PrimitiveComponent))
  (Rendering|Material|SetVectorParameterValue _returnvalue "GlassColor" PlayerColor :!class /Script/Engine.MaterialInstanceDynamic))

(event Custom|MulticastSetHood
  (params (Mesh :type Skeletal%20Mesh%20Object%20Reference) (Material :type Material%20Instance%20Object%20Reference) (Color :type Array%20of%20Linear%20Color%20Structures))
  ;[1 1 0] Hood
  (Utilities|MacSetSkelethalMesh (Variables|Default|GetSK_Hood) Mesh (Utilities|Array|MakeArray Material) Color (Utilities|Array|MakeArray "None") false))

(event Custom|MulticastSetChest
  (params (ChestColor :type Array%20of%20Linear%20Color%20Structures) (Mesh :type Skeletal%20Mesh%20Object%20Reference) (Material :type Array%20of%20Material%20Instance%20Object%20References))
  (bind _sk_chest (Variables|Default|GetSK_Chest))
  ;[0 1 0] Chest Customization
  (Class|SkinnedMeshComponent|SetSkeletalMesh _sk_chest Mesh true)
  (for (_array_element _array_index) Material
    (bind _returnvalue (Rendering|Material|CreateDynamicMaterialInstance _sk_chest _array_element :!class /Script/Engine.KismetMaterialLibrary))
    (for (_array_element_2 _array_index_2) ChestColor
      (Rendering|Material|SetVectorParameterValue _returnvalue (Utilities|Array|Get(acopy) (Utilities|Array|MakeArray "RedHsl" "GreenHSL" "BlueHSL" "BlackHSL") _array_index_2) _array_element_2 :!class /Script/Engine.MaterialInstanceDynamic))
    (Rendering|Material|SetMaterial _sk_chest _array_index _returnvalue)))

(event Custom|ServerSetRangeWeapon
  ;[1 1 0] Switch to range weapon
  (switch int (Variables|Weapon|GetWeaponState) ; 0: None, 1: Melee, 2: Range
    (:0
      _)
    (:1
      _))
  (CallFunction|MulticastSetRangeWeapon)
  (Variables|BowState|SetbBowHidden false)
  (Variables|Weapon|SetWeaponState 2))

(event Custom|ServerSetNoWeapon
  ;[1 1 0] Switch to no weapon
  (switch int (Variables|Weapon|GetWeaponState) ; 0: None, 1: Melee, 2: Range
    (:1
      _)
    (:2
      (CallFunction|MulticastSetBowHidden)
      (Variables|BowState|SetbBowHidden true)))
  (Variables|Weapon|SetWeaponState 0))

(event Custom|MulticastSetFace
  (params (Face :type Struct%20Human%20Face%20and%20Proportion%20Structure))
  ;[0 1 0] Face and proportion
  (Utilities|MacSetFaceandProportion Face))

(event Custom|MulticastSetShoulder
  (params (TopColor :type Array%20of%20Linear%20Color%20Structures) (Mesh :type Skeletal%20Mesh%20Object%20Reference) (Material :type Material%20Instance%20Object%20Reference))
  (bind _sk_shoulders (Variables|Default|GetSK_Shoulders))
  ;[1 1 0] Shoulder
  (Class|SkinnedMeshComponent|SetSkeletalMesh _sk_shoulders Mesh true)
  (bind _returnvalue (Rendering|Material|CreateDynamicMaterialInstance _sk_shoulders Material :!class /Script/Engine.KismetMaterialLibrary))
  (for (_array_element _array_index) TopColor
    (Rendering|Material|SetVectorParameterValue _returnvalue (Utilities|Array|Get(acopy) (Utilities|Array|MakeArray "RedHsl" "GreenHSL" "BlueHSL") _array_index) _array_element :!class /Script/Engine.MaterialInstanceDynamic))
  (Rendering|Material|SetMaterial _sk_shoulders 0 _returnvalue))

(event Custom|MulticastSetGloves
  (params (Mesh :type Skeletal%20Mesh%20Object%20Reference) (Material :type Material%20Instance%20Object%20Reference) (GlovesColor :type Array%20of%20Linear%20Color%20Structures))
  ;[1 1 0] Gloves
  (Utilities|MacSetSkelethalMesh (Variables|Default|GetSK_Gloves) Mesh (Utilities|Array|MakeArray Material) GlovesColor (Utilities|Array|MakeArray "None") false))

(event Custom|MulticastSetHelmet
  (params (Mesh :type Skeletal%20Mesh%20Object%20Reference) (Material :type Material%20Instance%20Object%20Reference) (Color :type Array%20of%20Linear%20Color%20Structures))
  ;[1 1 0] Helmet
  (Utilities|MacSetSkelethalMesh (Variables|Default|GetSK_Helmet) Mesh (Utilities|Array|MakeArray Material) Color (Utilities|Array|MakeArray "None") false))

(event Custom|MulticastSetBoots
  (params (BootsColor :type Linear%20Color%20Structure) (Mesh :type Skeletal%20Mesh%20Object%20Reference) (Material :type Material%20Instance%20Object%20Reference))
  (bind _sk_boots (Variables|Default|GetSK_Boots))
  ;[0 1 0] Boots Customization
  (Class|SkinnedMeshComponent|SetSkeletalMesh _sk_boots Mesh true)
  (bind _returnvalue (Rendering|Material|CreateDynamicMaterialInstance _sk_boots Material :!class /Script/Engine.KismetMaterialLibrary))
  (Rendering|Material|SetVectorParameterValue _returnvalue "HSL" BootsColor :!class /Script/Engine.MaterialInstanceDynamic)
  (Rendering|Material|SetMaterial _sk_boots 0 _returnvalue))

(event Custom|MulticastSetRangeWeapon
  ;[1 1 0] Switch to range weapon
  (Rendering|SetVisibility (Variables|Default|GetFP_Gun) true false)
  (Animation|Montage|MontagePlay (Components|SkeletalMesh|GetAnimInstance (Variables|Default|GetMesh2P)) (Utilities|Array|Get(acopy) (Variables|BowMontage|GetUnholsterArmsAnims)) 1.0 "MontageLength" 0.0)
  (Variables|BowState|SetbBowHidden false)
  (Variables|Weapon|SetWeaponState 2))

(event Custom|MulticastSetShild
  ;[1 1 0] Shild
)

(event Custom|MulticastSetPants
  (params (PantsColor :type Linear%20Color%20Structure) (Mesh :type Skeletal%20Mesh%20Object%20Reference) (Material :type Material%20Instance%20Object%20Reference))
  (bind _sk_pants (Variables|Default|GetSK_Pants))
  ;[0 1 0] Pants Customization
  (Class|SkinnedMeshComponent|SetSkeletalMesh _sk_pants Mesh true)
  (bind _returnvalue (Rendering|Material|CreateDynamicMaterialInstance _sk_pants Material :!class /Script/Engine.KismetMaterialLibrary))
  (Rendering|Material|SetVectorParameterValue _returnvalue "HSL" PantsColor :!class /Script/Engine.MaterialInstanceDynamic)
  (Rendering|Material|SetMaterial _sk_pants 0 _returnvalue))

(event Custom|MulticastSetMeleeWeapon
  ;[1 1 0] Melee weapon
)

(event Custom|MulticastSetHair
  (params (HairColor :type Linear%20Color%20Structure) (HairMesh :type Skeletal%20Mesh%20Object%20Reference) (BeardMesh :type Skeletal%20Mesh%20Object%20Reference) (HairMaterial :type Material%20Instance%20Object%20Reference) (BeardMaterial :type Material%20Instance%20Object%20Reference))
  (bind _sk_beard (Variables|Default|GetSK_Beard))
  (bind _sk_hair (Variables|Default|GetSK_Hair))
  ;[0 1 0] Hair and beard
  (Class|SkinnedMeshComponent|SetSkeletalMesh _sk_hair HairMesh true)
  (bind _returnvalue (Rendering|Material|CreateDynamicMaterialInstance _sk_hair HairMaterial :!class /Script/Engine.KismetMaterialLibrary))
  (Rendering|Material|SetVectorParameterValue _returnvalue "TipColor" HairColor :!class /Script/Engine.MaterialInstanceDynamic)
  (Rendering|Material|SetMaterial _sk_hair 0 _returnvalue)
  (Rendering|Material|SetMaterial _sk_hair 1 _returnvalue)
  (Class|SkinnedMeshComponent|SetSkeletalMesh _sk_beard BeardMesh true)
  (bind _returnvalue_2 (Rendering|Material|CreateDynamicMaterialInstance _sk_beard BeardMaterial :!class /Script/Engine.KismetMaterialLibrary))
  (Rendering|Material|SetVectorParameterValue _returnvalue_2 "TipColor" HairColor :!class /Script/Engine.MaterialInstanceDynamic)
  (Rendering|Material|SetMaterial _sk_beard 0 _returnvalue_2))

(event Custom|MulticastSetOrgans
  (params (SkelethalOrgan :type Array%20of%20Struct%20Skelethal%20Organ%20Structures) (StaticOrgan :type Array%20of%20Struct%20Static%20Organ%20Structures) (Face :type Struct%20Human%20Face%20and%20Proportion%20Structure))
  ;[1 1 0] Set Default Organ
  (Utilities|MacSetInitialOrgans (Utilities|Array|MakeArray (Variables|Default|GetSK_Chest) (Variables|Default|GetSK_Pants) (Variables|Default|GetSK_Boots) (Variables|Default|GetSK_Hair) (Variables|Default|GetSK_Beard) (Variables|Default|GetSK_Shoulders) (Variables|Default|GetSK_Gloves) (Variables|Default|GetSK_Helmet)) SkelethalOrgan (Utilities|Array|MakeArray (Variables|Default|GetSM_Sword) (Variables|Default|GetSM_Shild)) StaticOrgan)
  (Utilities|MacSetFaceandProportion Face))

(event Custom|MulticastSetBowHidden
  ;[1 1 0] Switch to no weapon
  (Animation|Montage|MontagePlay (Components|SkeletalMesh|GetAnimInstance (Variables|Default|GetMesh2P)) (Utilities|Array|Get(acopy) (Variables|BowMontage|GetHolsterArmsAnims)) 1.0 "MontageLength" 0.0)
  (Variables|BowState|SetbBowHidden true)
  (Variables|Weapon|SetWeaponState 0))

(event Custom|TurnBody
  (params (AxisValue :type Float%20%28single-precision%29))
  (bind _returnvalue (Pawn|GetControlRotation :!class /Script/Engine.Pawn))
  (bind _slowratenormal (Variables|CharacterRotation|GetSlowRateNormal))
  (bind _yaw (Math|Rotator|BreakRotator _returnvalue))
  (bind _returnvalue_2 (/ AxisValue _slowratenormal))
  (bind _returnvalue_3 (Math|Rotator|MakeRotator 0.0 0.0 _yaw))
  ;[0 1 0] Turn and lookup
  (Pawn|Input|AddControllerYawInput _returnvalue_2)
  (Transformation|SetActorRotation _returnvalue_3)
  (CallFunction|ServerReplicateTurnBody _returnvalue_2 _returnvalue_3))

(event Custom|MulticastRun
  ;[1 1 0] Toggle between Walk and Run
  (Variables|/Script/Engine.CharacterMovementComponent|SetMaxWalkSpeed (Variables|Character|GetCharacterMovement) (Variables|DefaultValue|GetDefaultRunSpeed)))

(event Custom|ServerReplicateTurnBody
  (params (AxisValue :type Float%20%28single-precision%29) (ActorRotation :type Rotator))
  ;[0 1 0] Turn and lookup
  (CallFunction|MulticastReplicateTurnBody AxisValue ActorRotation))

(event Custom|MulticastWalk
  ;[1 1 0] Toggle between Walk and Run
  (Variables|/Script/Engine.CharacterMovementComponent|SetMaxWalkSpeed (Variables|Character|GetCharacterMovement) (Variables|DefaultValue|GetDefaultWalkSpeed)))

(event Custom|ServerWalk
  ;[1 1 0] Toggle between Walk and Run
  (CallFunction|MulticastWalk))

(event Custom|MoveBody
  (params (AxisValue :type Float%20%28single-precision%29) (Direction :type String))
  ;[0 1 0] Movement
  (Pawn|Input|AddMovementInput (Class|LordsOfCaladanFunctionLibrary|GetMovementVector (Class|LordsOfCaladanFunctionLibrary|MakeRotatorbyZ (Pawn|GetControlRotation :!class /Script/Engine.Pawn)) Direction) AxisValue false))

(event Custom|MulticastReplicateTurnBody
  (params (AxisValue :type Float%20%28single-precision%29) (ActorRotation :type Rotator))
  ;[0 1 0] Turn and lookup
  (Pawn|Input|AddControllerYawInput AxisValue)
  (Transformation|SetActorRotation ActorRotation))

(event Custom|LookupBody
  (params (AxisValue :type Float%20%28single-precision%29))
  ;[0 1 0] Turn and lookup
  (Pawn|Input|AddControllerPitchInput (/ AxisValue (Variables|CharacterRotation|GetSlowRateNormal))))

(event Custom|SetActiveCamera
  (params (CamIndex :type Integer))
  (bind _rtscamera (Variables|Default|GetRTSCamera))
  (bind _tpscamera (Variables|Default|GetTPSCamera))
  ;[1 1 0] SetActiveCamera
  (switch int CamIndex ; FPS=1, RTS=2, TPS=3
    (:1
      (Utilities|MacActivateFPS _tpscamera))
    (:2
      (Utilities|MacActivateRTSorTPS (Variables|Default|GetFPSCamera) _rtscamera))
    (:3
      (Utilities|MacActivateRTSorTPS _rtscamera _tpscamera))))

(event Custom|Walk
  ;[1 1 0] Toggle between Walk and Run
  (Variables|/Script/Engine.CharacterMovementComponent|SetMaxWalkSpeed (Variables|Character|GetCharacterMovement) (Variables|DefaultValue|GetDefaultWalkSpeed))
  (CallFunction|ServerWalk))

(event Custom|Run
  ;[1 1 0] Toggle between Walk and Run
  (Variables|/Script/Engine.CharacterMovementComponent|SetMaxWalkSpeed (Variables|Character|GetCharacterMovement) (Variables|DefaultValue|GetDefaultRunSpeed))
  (CallFunction|ServerRun))

(event Custom|ServerRun
  ;[1 1 0] Toggle between Walk and Run
  (CallFunction|MulticastRun))

(event Custom|RTSCameraRotateY
  (params (AxisValue :type Float%20%28single-precision%29))
  (bind _rtscamera (Variables|Default|GetRTSCamera))
  (bind _relativerotation (Variables|/Script/Engine.SceneComponent|GetRelativeRotation _rtscamera))
  (bind (_roll _pitch _yaw) (Math|Rotator|BreakRotator _relativerotation))
  ;[0 1 0] RTS Camera Rotation
  (Transformation|SetRelativeRotation _rtscamera (Math|Rotator|MakeRotator _roll (+ (* AxisValue (Variables|RTSCamera|GetRotationSpeed) -1.0) _pitch) _yaw) false false))

(event Custom|RTSCameraMoveRight
  (params (AxisValue :type Float%20%28single-precision%29))
  (bind _rtscamera (Variables|Default|GetRTSCamera))
  (bind _relativerotation (Variables|/Script/Engine.SceneComponent|GetRelativeRotation _rtscamera))
  (bind _returnvalue (Math|Rotator|GetRotationXVector _relativerotation))
  (bind (_x _y) (Math|Vector|BreakVector _returnvalue))
  ;[0 1 0] RTS Camera movement
  (Transformation|SetRelativeLocation _rtscamera (+ (* (Math|Vector|MakeVector (* _y -1.0) _x 0.0) (* AxisValue (Variables|RTSCamera|GetMoveSpeed))) (Variables|/Script/Engine.SceneComponent|GetRelativeLocation _rtscamera)) false false))

(event Custom|RTSCameraRotateZ
  (params (AxisValue :type Float%20%28single-precision%29))
  (bind _rtscamera (Variables|Default|GetRTSCamera))
  (bind _relativerotation (Variables|/Script/Engine.SceneComponent|GetRelativeRotation _rtscamera))
  (bind (_roll _pitch _yaw) (Math|Rotator|BreakRotator _relativerotation))
  ;[0 1 0] RTS Camera Rotation
  (Transformation|SetRelativeRotation _rtscamera (Math|Rotator|MakeRotator _roll _pitch (+ (* AxisValue (Variables|RTSCamera|GetRotationSpeed)) _yaw)) false false))

(event Custom|RTSCameraMoveForward
  (params (AxisValue :type Float%20%28single-precision%29))
  (bind _rtscamera (Variables|Default|GetRTSCamera))
  ;[0 1 0] RTS Camera movement
  (Transformation|SetRelativeLocation _rtscamera (+ (* (Math|Rotator|GetRotationXVector (Variables|/Script/Engine.SceneComponent|GetRelativeRotation _rtscamera)) (* AxisValue (Variables|RTSCamera|GetMoveSpeed))) (Variables|/Script/Engine.SceneComponent|GetRelativeLocation _rtscamera)) false false))

(fn ConstructionScript
  (Variables|RTSCamera|SetRTSMeshes (Utilities|Array|MakeArray (Variables|Character|GetMesh) (Variables|Default|GetSK_Chest) (Variables|Default|GetSK_Pants) (Variables|Default|GetSK_Boots) (Variables|Default|GetSK_Beard) (Variables|Default|GetSK_Hair) (Variables|Default|GetSK_Body) (Variables|Default|GetSK_Jaw) (Variables|Default|GetSK_Shoulders) (Variables|Default|GetSK_Gloves) (Variables|Default|GetSK_Helmet) (Variables|Default|GetSK_Hood)))
  (for _array_element (Utilities|Array|MakeArray (Variables|Default|GetSM_Sword) (Variables|Default|GetSM_Shild))
    (Utilities|Array|Add (Variables|RTSCamera|GetRTSMeshes) _array_element))
  (Variables|FPSCamera|SetFPSMeshes (Utilities|Array|MakeArray (Variables|Default|GetTpsMesh)))
  (Class|SkinnedMeshComponent|SetMasterPoseComponent (Variables|Default|GetSK_Chest) (Variables|Character|GetMesh))
  (Transformation|AttachComponentToComponent (Variables|Default|GetLeftArmColl) (Variables|Default|GetSK_Body) "hand_l" "KeepRelative" "KeepRelative" "KeepRelative" true))