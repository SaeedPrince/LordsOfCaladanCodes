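; FighterBP is a player fighter character with camera-relative movement and mouse-steered sword and shield poses.
; While attacking or defending, turn and lookup input accumulate into FireTurn and FireLookup through server-named save events, clamped per stance.
; Yaw always rotates the body, while pitch moves the view only outside both stances.
; A multicast-named event messages the AnimInstance for attack poses, but the attack-start chain and cooldown are unfinished stubs.
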(event Custom|TurnPlayer
  (params (AxisValue :type Float%20%28single-precision%29))
  ;[1 1 0] Mouse move: Body rotation, Sword and shild movement
  (if (Variables|State|GetIsAttacking)
    (Variables|Mouse|SetTurnCase "Attack")
    (CallFunction|SaveTurnonServer (Variables|Mouse|GetTurnCase) AxisValue :!label _label)
    (elif (Variables|State|GetIsDefending)
      (Variables|Mouse|SetTurnCase "Defend")
      (goto _label)
      (else
        _)))
  (Pawn|Input|AddControllerYawInput AxisValue)
  (Transformation|SetActorRotation (Math|Rotator|MakeRotator 0.0 0.0 (.Yaw (Math|Rotator|BreakRotator (Pawn|GetControlRotation :!class /Script/Engine.Pawn))))))

(event Custom|MulticastPlayerAttackPoseStart
  ;[1 1 0] Attack Player
  (Class|MyInterface|InterfaceAttackPoseOnce(Message) (Components|SkeletalMesh|GetAnimInstance (Variables|Character|GetMesh))))

(event Custom|PlayerAttackPoseStart
  ;[1 1 0] Attack Player
  (if (not (Variables|State|GetIsAttacking))
    (if (not (Variables|State|GetIsDefending))
      _)))

(event Custom|ServerPlayerAttackPoseStart
  ;[1 1 0] Attack Player
)

(event Custom|SaveTurnOnServer
  (params (Case :type String) (Turn :type Float%20%28single-precision%29))
  ;[1 1 0] Mouse move: Body rotation, Sword and shild movement
  (switch string Case
    (:Attack
      (Variables|Mouse|SetFireTurn (Class|LordsOfCaladanFunctionLibrary|ClampFloat (+ Turn (Variables|Mouse|GetFireTurn)) (Variables|Mouse|GetMinAttackTurn) (Variables|Mouse|GetMaxAttackTurn))))
    (:Defend
      (Variables|Mouse|SetFireTurn (Class|LordsOfCaladanFunctionLibrary|ClampFloat (+ Turn (Variables|Mouse|GetFireTurn)) (Variables|Mouse|GetMinDefendTurn) (Variables|Mouse|GetMaxDefendTurn))))))

(event Custom|LookupPlayer
  (params (AxisValue :type Float%20%28single-precision%29))
  ;[1 1 0] Mouse move: Body rotation, Sword and shild movement
  (if (Variables|State|GetIsAttacking)
    (Variables|Mouse|SetLookupCase "Attack")
    (CallFunction|SaveLookuponServer (Variables|Mouse|GetLookupCase) AxisValue :!label _label)
    (elif (Variables|State|GetIsDefending)
      (Variables|Mouse|SetLookupCase "Defend")
      (goto _label)
      (else
        (Pawn|Input|AddControllerPitchInput AxisValue)))))

(event Custom|SaveLookupOnServer
  (params (Case :type String) (Lookup :type Float%20%28single-precision%29))
  ;[1 1 0] Mouse move: Body rotation, Sword and shild movement
  (switch string Case
    (:Attack
      (Variables|Mouse|SetFireLookup (Class|LordsOfCaladanFunctionLibrary|ClampFloat (+ Lookup (Variables|Mouse|GetFireLookup)) (Variables|Mouse|GetMinAttackLookup) (Variables|Mouse|GetMaxAttackLookup))))
    (:Defend
      (Variables|Mouse|SetFireLookup (Class|LordsOfCaladanFunctionLibrary|ClampFloat (+ Lookup (Variables|Mouse|GetFireLookup)) (Variables|Mouse|GetMinDefendLookup) (Variables|Mouse|GetMaxDefendLookup))))))

(event Custom|PlayerMove
  (params (AxisValue :type Float%20%28single-precision%29) (Direction :type String))
  (Pawn|Input|AddMovementInput (Class|LordsOfCaladanFunctionLibrary|GetMovementVector (Class|LordsOfCaladanFunctionLibrary|MakeRotatorbyZ (Pawn|GetControlRotation :!class /Script/Engine.Pawn)) Direction) AxisValue false))

(fn ConstructionScript)

(fn AttackPoseCooldown)