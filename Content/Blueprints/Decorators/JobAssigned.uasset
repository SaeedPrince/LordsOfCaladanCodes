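; JobAssigned is a behavior tree decorator, named for a job-assignment condition on human AI, whose check currently always returns false.
; PerformConditionCheck runs a macro that lazily caches the owner as AIController_Game and its controlled pawn as HumanBP.
; No job state is read, so the cached references do not yet affect the result.
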(fn PerformConditionCheck
  (params (OwnerActor :type Actor%20Object%20Reference))
  (Utilities|MacSetGameObject OwnerActor true true)
  (return false))