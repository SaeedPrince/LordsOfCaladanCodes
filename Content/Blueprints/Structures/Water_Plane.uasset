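; Water_Plane is a placeable water surface actor with a plane mesh and an optional planar reflection.
; The construction script scales both the plane and the reflection component from SizeX and SizeY, each with its own base-size divisor.
; It also applies the WaterMaterial to the plane and toggles reflection visibility through UseInternalReflectionPlane.
; The event graph has no active logic, so all setup happens at construction.
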(event EventBeginPlay)

(event Collision|EventActorBeginOverlap
  (params (OtherActor :type Actor%20Object%20Reference)))

(event EventTick
  (params (DeltaSeconds :type Float%20%28single-precision%29)))

(fn ConstructionScript
  (bind _planarreflection (Variables|Default|GetPlanarReflection))
  (bind _plane (Variables|Default|GetPlane))
  (bind _size_x (Variables|Default|GetSize%20X))
  (bind _size_y (Variables|Default|GetSize%20Y))
  (Rendering|SetVisibility _planarreflection (Variables|Default|GetUse%20Internal%20Reflection%20Plane) false)
  (Transformation|SetRelativeScale3D _planarreflection (Math|Vector|MakeVector (/ _size_x 4e+03) (/ _size_y 4e+03) 1.0))
  (Transformation|SetRelativeScale3D _plane (Math|Vector|MakeVector (/ _size_x 1e+02) (/ _size_y 1e+02) 1.0))
  (Rendering|Material|SetMaterial _plane 0 (Variables|Default|GetWater%20Material)))