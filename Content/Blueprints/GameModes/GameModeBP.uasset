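; Game mode Blueprint that spawns player characters at random Ally or Enemy start points.
; SavePlayerStartRefs sorts all PlayerStart actors into per-team arrays, which RandomSpawnTransform draws from to build a spawn transform.
; CreateNewCharacter runs only with authority: it spawns the given class there, sets its team type, has the controller possess it, cross-links both references and reports success.
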(event Custom|SavePlayerStartRefs
  (bind _outactors (Actor|GetAllActorsOfClass "/Script/Engine.PlayerStart"))
  (for _array_element _outactors
    (switch string (Class|LordsOfCaladanFunctionLibrary|GetPlayerStartType _array_element)
      (:Ally
        (Utilities|Array|Add (Variables|PlayerStart|GetStartAlly) _array_element))
      (:Enemy
        (Utilities|Array|Add (Variables|PlayerStart|GetStartEnemy) _array_element)))))

(fn ConstructionScript)

(fn CreateNewCharacter
  (params (CharacterClass :type Medieval%20Warrior%20Class%20Reference) (Type :type String) (ControllerRef :type Player%20Controller%20Game%20Object%20Reference))
  (Networking|SwitchHasAuthority
    (:Authority
      (Utilities|IsValid ControllerRef
        (:Is%20Valid
          (bind _returnvalue (Game|SpawnActorfromClass CharacterClass (CallFunction|RandomSpawnTransform Type) "Undefined" ControllerRef 0))
          (Utilities|IsValid _returnvalue
            (:Is%20Valid
              (LocalVariables|SetResult true)
              (Class|Fighter|SetType _returnvalue Type)
              (Class|Fighter|SetRunner _returnvalue "Player")
              (Pawn|Possess ControllerRef _returnvalue)
              (Variables|/Game/Blueprints/Controllers/PlayerController_Game.PlayerController_Game_C|SetCharacterRef ControllerRef _returnvalue)
              (Variables|/Game/Blueprints/Characters/FighterBP.FighterBP_C|SetControllerRef _returnvalue ControllerRef))
            (:Is%20Not%20Valid
              (LocalVariables|SetResult false :!label _label))))
        (:Is%20Not%20Valid
          (goto _label))))
    (:Remote
      (goto _label)))
  (return (LocalVariables|GetResult)))

(fn RandomSpawnTransform
  (params (Type :type String))
  (switch string Type
    (:Ally
      (LocalVariables|SetLocalArray (Variables|PlayerStart|GetStartAlly)))
    (:Enemy
      (LocalVariables|SetLocalArray (Variables|PlayerStart|GetStartEnemy))))
  (return (Math|Transform|MakeTransform (.Location (CallFunction|GetRandomLocation (LocalVariables|GetLocalArray))) (.Rotation (CallFunction|GetRandomLocation (LocalVariables|GetLocalArray))))))

(fn GetRandomLocation
  (params (StartArray :type Array%20of%20Player%20Start%20Object%20References))
  (bind _returnvalue (Utilities|Array|Length StartArray))
  (bind _returnvalue_2 (- _returnvalue 1))
  (bind _returnvalue_3 (Math|Random|RandomIntegerinRange 0 _returnvalue_2))
  (bind _output (Utilities|Array|Get(acopy) StartArray _returnvalue_3))
  (bind (_location _rotation) (CallFunction|GetLocation _output))
  (return _location _rotation))

(fn GetLocation
  (params (PlayerStart :type Player%20Start%20Object%20Reference))
  (bind _returnvalue (Transformation|GetActorTransform PlayerStart))
  (bind (_location _rotation) (Math|Transform|BreakTransform _returnvalue))
  (return _location _rotation))