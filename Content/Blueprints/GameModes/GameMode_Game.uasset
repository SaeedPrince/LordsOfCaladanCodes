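; Server game mode that spawns and possesses player characters at cached PlayerStarts, and can spawn AI humans and armories.
; New player characters get randomized faces, body proportions, clothing, hair and gear from mesh/material arrays, pushed via multicast.
; Helpers draw player colors, usernames and spawn places from shrinking pools.
; StartServer spawns the sky dome and starts a one-second timer advancing server time and virtual time at separate day/night rates.
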(event Custom|InitializeServer
  ;[0 1 0] Initialize Server
  (Utilities|MacSavePlayerStartRefs))

(event Custom|StartServer
  (bind _zerotime (Variables|ServerStats|GetZeroTime))
  ;[1 1 0] Start Server
  (Variables|ServerStats|SetServerTime _zerotime)
  (Variables|ServerStats|SetVirtualTime _zerotime)
  (bind _returnvalue (Utilities|Time|SetTimerbyFunctionName self "ServerTimeUpdate" 1.0 true))
  (Variables|ServerStats|SetTimerServerTimeUpdate _returnvalue)
  (bind _returnvalue_2 (Game|SpawnActorfromClass "/Game/Blueprints/Environment/Sky/BP_DayCycle_SkyDome.BP_DayCycle_SkyDome_C" (Math|Transform|MakeTransform "0, 0, 0") "Undefined" 0 0))
  (Utilities|IsValid _returnvalue_2
    (:Is%20Valid
      (Variables|Sky|SetSkyReference _returnvalue_2)
      (Development|PrintString "Sky created" true true "(R=0.000000,G=1.000000,B=0.000000,A=1.000000)" 8.0))
    (:Is%20Not%20Valid
      (Development|PrintString "Sky not created" true true "(R=1.000000,G=0.000000,B=0.000000,A=1.000000)" 8.0))))

(fn ConstructionScript)

(fn CreateNewCharacter
  (params (CharacterClass :type Human%20BP%20Class%20Reference) (ControllerRef :type Player%20Controller%20Game%20Object%20Reference) (PlayerColor :type Linear%20Color%20Structure) (Place :type Integer))
  (bind (_skelethalarray _staticarray) (CallFunction|DefaultHumanOrgans))
  (bind _humanface (CallFunction|DefaultHumanFaceandProportion))
  (bind _playerstartarray (Variables|ServerInitial|GetPlayerStartArray))
  (bind _output (Utilities|Array|Get(acopy) _playerstartarray Place))
  (Networking|SwitchHasAuthority
    (:Authority
      (Utilities|IsValid ControllerRef
        (:Is%20Valid
          (bind _returnvalue (Game|SpawnActorfromClass CharacterClass (Math|Transform|MakeTransform (Transformation|GetActorLocation _output) (Transformation|GetActorRotation _output)) "Undefined" ControllerRef 0))
          (Utilities|IsValid _returnvalue
            (:Is%20Valid
              (LocalVariables|SetResult true)
              (Pawn|Possess ControllerRef _returnvalue)
              (Variables|/Game/Blueprints/Controllers/PlayerController_Game.PlayerController_Game_C|SetCharacterRef ControllerRef _returnvalue)
              (Variables|/Game/Blueprints/Characters/HumanBP.HumanBP_C|SetControllerRef _returnvalue ControllerRef)
              (Default|MulticastSetOrgans _returnvalue _skelethalarray _staticarray _humanface)
              (Default|SetOrgans _returnvalue _skelethalarray _staticarray _humanface)
              (Variables|/Game/Blueprints/Controllers/PlayerController_Game.PlayerController_Game_C|SetPlayerColor ControllerRef PlayerColor)
              (bind _outactors (Actor|GetAllActorsOfClass "/Game/Blueprints/Characters/HumanBP.HumanBP_C"))
              (for _array_element _outactors
                (Default|SetPlayerColorforEveryone _array_element (Variables|/Game/Blueprints/Controllers/PlayerController_Game.PlayerController_Game_C|GetPlayerColor (Variables|/Game/Blueprints/Characters/HumanBP.HumanBP_C|GetControllerRef _array_element)))
                (Utilities|Array|RemoveItem (Variables|ServerInitial|GetAvailableColors) PlayerColor)))
            (:Is%20Not%20Valid
              (LocalVariables|SetResult false :!label _label))))
        (:Is%20Not%20Valid
          (goto _label))))
    (:Remote
      (goto _label)))
  (return (LocalVariables|GetResult)))

(fn RandomSpawnTransformbyType
  (params (Type :type String))
  (switch string Type
    (:Ally
      (LocalVariables|SetLocalArray (Variables|PlayerStart|GetStartAlly)))
    (:Enemy
      (LocalVariables|SetLocalArray (Variables|PlayerStart|GetStartEnemy))))
  (return (Math|Transform|MakeTransform (.Location (CallFunction|GetRandomLocation (LocalVariables|GetLocalArray))) (.Rotation (CallFunction|GetRandomLocation (LocalVariables|GetLocalArray))))))

(fn GetRandomLocation
  (params (StartArray :type Array%20of%20Player%20Start%20Object%20References))
  (bind _returnvalue (Utilities|Array|Length StartArray))
  (bind _returnvalue_2 (- _returnvalue 1))
  (bind _returnvalue_3 (Math|Random|RandomIntegerinRange 0 _returnvalue_2))
  (bind _output (Utilities|Array|Get(acopy) StartArray _returnvalue_3))
  (bind (_location _rotation) (CallFunction|GetLocation _output))
  (return _location _rotation))

(fn GetLocation
  (params (PlayerStart :type Player%20Start%20Object%20Reference))
  (bind _returnvalue (Transformation|GetActorTransform PlayerStart))
  (bind (_location _rotation) (Math|Transform|BreakTransform _returnvalue))
  (return _location _rotation))

(fn GetRandomUsername
  (bind _availableusernames (Variables|ServerInitial|GetAvailableUsernames))
  (bind _output_get (LocalVariables|Setout (Utilities|Array|Get(acopy) _availableusernames (Math|Random|RandomIntegerinRange 0 (- (Utilities|Array|Length _availableusernames) 1)))))
  (Utilities|Array|RemoveItem _availableusernames _output_get)
  (return (LocalVariables|Getout)))

(fn ReadytoStart
  (bind _gamereadychecked (Variables|Players|GetGameReadyChecked))
  (return (and (Utilities|Array|Get(acopy) _gamereadychecked) (Utilities|Array|Get(acopy) _gamereadychecked 1))))

(fn GetRandomPlayerColor
  (bind _availablecolors (Variables|ServerInitial|GetAvailableColors))
  (bind _output_get (LocalVariables|Setout (Utilities|Array|Get(acopy) _availablecolors (Math|Random|RandomIntegerinRange 0 (- (Utilities|Array|Length _availablecolors) 1)))))
  (Utilities|Array|RemoveItem _availablecolors _output_get)
  (return (LocalVariables|Getout)))

(fn GetSpawnPlacebyOrder
  (bind _availableplaces (Variables|ServerInitial|GetAvailablePlaces))
  (bind _output_get (LocalVariables|Setout (Utilities|Array|Get(acopy) _availableplaces)))
  (Utilities|Array|RemoveItem _availableplaces _output_get)
  (return (LocalVariables|Getout)))

(fn SpawnHouse
  (params (SpawnLocation :type Vector) (SpawnRotation :type Rotator))
  (bind _returnvalue (Game|SpawnActorfromClass "/Game/Assets/BP_Meshes/Architecture/BP_Armory.BP_Armory_C" (Math|Transform|MakeTransform SpawnLocation SpawnRotation) "AlwaysSpawn" 0 0))
  (Utilities|IsValid _returnvalue
    (:Is%20Valid
      (Development|PrintString "Spawned" true true "(R=0.000000,G=1.000000,B=0.000000,A=1.000000)" 8.0))
    (:Is%20Not%20Valid
      (Development|PrintString "Not spawned" true true "(R=1.000000,G=0.000000,B=0.000000,A=1.000000)" 8.0))))

(fn ServerTimeUpdate
  (Variables|ServerStats|SetServerTime (+ (Variables|ServerStats|GetServerTime) (Math|Timespan|MakeTimespan 0 0 0 1)))
  (if (or (< (Class|KismetMathLibrary|GetHour (Variables|ServerStats|GetVirtualTime)) 7) (> (Class|KismetMathLibrary|GetHour (Variables|ServerStats|GetVirtualTime)) 17))
    (LocalVariables|SetVirtualAdd (Math|Timespan|MakeTimespan 0 0 0 (Variables|ServerStats|GetNightTimeScale)))
    (else
      (LocalVariables|SetVirtualAdd (Math|Timespan|MakeTimespan 0 0 0 (Variables|ServerStats|GetDayTimeScale)))))
  (bind _output_get (Variables|ServerStats|SetVirtualTime (+ (Variables|ServerStats|GetVirtualTime) (LocalVariables|GetVirtualAdd)))))

(fn SpawnAIHuman
  (params (Place :type Integer))
  (bind _playerstartarray (Variables|ServerInitial|GetPlayerStartArray))
  (bind _output (Utilities|Array|Get(acopy) _playerstartarray Place))
  (Networking|SwitchHasAuthority
    (:Authority
      (bind _returnvalue (AI|SpawnAIFromClass "/Game/Blueprints/Characters/HumanBP.HumanBP_C" "/Game/Blueprints/BehaviorTree/BT_Human.BT_Human" (Transformation|GetActorLocation _output) (Transformation|GetActorRotation _output) false))
      (Utilities|IsValid _returnvalue
        (:Is%20Valid
          (LocalVariables|SetOK true)
          (Utilities|Casting|CastToHumanBP _returnvalue))
        (:Is%20Not%20Valid
          (LocalVariables|SetOK false :!label _label)
          (return (LocalVariables|GetOK)))))
    (:Remote
      (goto _label))))

(fn RandomChestColor
  (bind _returnvalue (Utilities|MacRandomColor 0.0 1.3 0.0 1.5 0.0 1.5))
  (return _returnvalue _returnvalue (Utilities|MacRandomColor 0.9 1.1 0.0 1.5 0.0 1.2)))

(fn CreateHumanChest
  (bind (_chest _upperarm _lowerarm) (CallFunction|RandomChestColor))
  (bind _chests (Variables|CharacterCustomization|GetChests))
  (bind _defaulthumanchesttype (Variables|CharacterDefault|GetDefaultHumanChestType))
  (bind _defaulthumanchestmodel (Variables|CharacterDefault|GetDefaultHumanChestModel))
  (bind _defaulthumanchestmaterial (Variables|CharacterDefault|GetDefaultHumanChestMaterial))
  (bind (_mesh _material) (Utilities|GetMeshMat _chests _defaulthumanchesttype _defaulthumanchestmodel _defaulthumanchestmaterial))
  (return _mesh (Utilities|Array|MakeArray _material (.Material (Utilities|GetMeshMat (Variables|CharacterCustomization|GetSkirt) 0 0 (Variables|CharacterDefault|GetDefaultHumanSkirtMaterial)))) (Utilities|Array|MakeArray _chest _upperarm _lowerarm "(R=1.000000,G=1.000000,B=1.000000,A=0.000000)")))

(fn CreateHumanPants
  (bind _returnvalue (Math|Random|RandomIntegerinRange 0 10))
  (bind _returnvalue_2 (Math|Random|RandomIntegerinRange 0 10))
  (bind _pants (Variables|CharacterCustomization|GetPants))
  (bind _returnvalue_3 (Utilities|GetRandomonLength _pants))
  (bind (_mesh _material) (Utilities|GetMeshMat _pants _returnvalue_3 _returnvalue _returnvalue_2))
  (return _mesh _material (CallFunction|RandomPantsColor)))

(fn RandomPantsColor
  (return (Utilities|MacRandomColor 0.0 1.0 0.0 1.2 0.0 1.5)))

(fn RandomBootsColor
  (return (Utilities|MacRandomColor 0.0 1.0 0.0 1.2 0.0 1.5)))

(fn CreateHumanBoots
  (bind _returnvalue (Math|Random|RandomIntegerinRange 0 10))
  (bind _returnvalue_2 (Math|Random|RandomIntegerinRange 0 10))
  (bind _boots (Variables|CharacterCustomization|GetBoots))
  (bind _returnvalue_3 (Utilities|GetRandomonLength _boots))
  (bind (_mesh _material) (Utilities|GetMeshMat _boots _returnvalue_3 _returnvalue _returnvalue_2))
  (return _mesh _material (CallFunction|RandomBootsColor)))

(fn CreateHumanHair
  (bind _returnvalue (Math|Random|RandomIntegerinRange 0 6))
  (bind _returnvalue_2 (Math|Random|RandomIntegerinRange 0 7))
  (bind _beards (Variables|CharacterCustomization|GetBeards))
  (bind _hairs (Variables|CharacterCustomization|GetHairs))
  (bind (_mesh _material) (Utilities|GetMeshMat _beards 0 _returnvalue_2))
  (bind (_mesh_2 _material_2) (Utilities|GetMeshMat _hairs 0 _returnvalue))
  (return _mesh_2 _mesh _material_2 _material (Utilities|Select :Index (Math|Random|RandomIntegerinRange 0 5) :Option%200 "(R=0.965000,G=0.702598,B=0.214586,A=1.000000)" :Option%201 "(R=0.040000,G=0.040000,B=0.040000,A=1.000000)" :Option%202 "(R=0.327778,G=0.127438,B=0.043735,A=1.000000)" :Option%203 "(R=0.695000,G=0.695000,B=0.695000,A=1.000000)" :Option%204 "(R=0.505000,G=0.095155,B=0.035350,A=1.000000)" :Option%205 "(R=0.095000,G=0.037655,B=0.012308,A=1.000000)")))

(fn DefaultHumanFaceandProportion
  (bind _returnvalue (Math|Random|RandomFloatinRange 0.0 0.15))
  (bind _returnvalue_2 (Math|Random|RandomFloatinRange 0.2 1.1))
  (bind _returnvalue_3 (Math|Random|RandomFloatinRange 0.0 2e+02))
  (bind _returnvalue_4 (Class|KismetMathLibrary|HSVtoRGB _returnvalue_3 _returnvalue _returnvalue_2 0.0))
  (return (Utilities|Struct|MakeStructHumanFaceAndProportion (* (Math|Random|RandomFloatinRange 0.7 1.7) (.V (Math|Color|RGBtoHSV(LinearColor) _returnvalue_4))) (Math|Random|RandomFloatinRange 0.0 1.0) (Math|Random|RandomFloatinRange -0.5 1.0) (Math|Random|RandomFloatinRange 1.0 1.3) (Math|Float|Clamp(Float) (Math|Random|RandomFloatinRange -1.0 2.0) 0.0 2.0) _returnvalue_4 (Math|Random|RandomFloatinRange -1.0 1.3) (Math|Random|RandomFloatinRange 0.85 1.2))))

(fn DefaultHumanOrgans
  (bind (_mesh _material _chestcolor) (CallFunction|CreateHumanChest))
  (bind (_mesh_2 _material_2 _color _parameter) (CallFunction|CreateSword))
  (bind (_mesh_3 _material_3 _color_2 _parameter_2) (CallFunction|CreateShield))
  (bind (_mesh_4 _material_4 _pantscolor) (CallFunction|CreateHumanPants))
  (bind (_mesh_5 _material_5 _bootscolor) (CallFunction|CreateHumanBoots))
  (bind (_hairmesh _beardmesh _hairmaterial _beardmaterial _haircolor) (CallFunction|CreateHumanHair))
  (bind (_mesh_6 _material_6 _shouldercolor _parameters) (CallFunction|CreateRandomShoulder))
  (bind (_mesh_7 _material_7 _glovescolor _parameters_2) (CallFunction|CreateRandomGloves))
  (bind (_mesh_8 _material_8 _helmetcolor _parameters_3) (CallFunction|CreateRandomHelmet))
  (bind _array (Utilities|Array|MakeArray "HSL"))
  (bind _array_2 (Utilities|Array|MakeArray "TipColor"))
  (bind _array_3 (Utilities|Array|MakeArray _haircolor))
  (return (Utilities|Array|MakeArray (Utilities|Struct|MakeStructSkelethalOrgan _mesh (Utilities|Struct|MakeStructMeshParameters _material _chestcolor (CallFunction|ChestParameters) true)) (Utilities|Struct|MakeStructSkelethalOrgan _mesh_4 (Utilities|Struct|MakeStructMeshParameters (Utilities|Array|MakeArray _material_4) (Utilities|Array|MakeArray _pantscolor) _array true)) (Utilities|Struct|MakeStructSkelethalOrgan _mesh_5 (Utilities|Struct|MakeStructMeshParameters (Utilities|Array|MakeArray _material_5) (Utilities|Array|MakeArray _bootscolor) _array true)) (Utilities|Struct|MakeStructSkelethalOrgan _hairmesh (Utilities|Struct|MakeStructMeshParameters (Utilities|Array|MakeArray _hairmaterial) _array_3 _array_2 true)) (Utilities|Struct|MakeStructSkelethalOrgan _beardmesh (Utilities|Struct|MakeStructMeshParameters (Utilities|Array|MakeArray _beardmaterial) _array_3 _array_2 true)) (Utilities|Struct|MakeStructSkelethalOrgan _mesh_6 (Utilities|Struct|MakeStructMeshParameters _material_6 _shouldercolor _parameters false)) (Utilities|Struct|MakeStructSkelethalOrgan _mesh_7 (Utilities|Struct|MakeStructMeshParameters _material_7 _glovescolor _parameters_2 false)) (Utilities|Struct|MakeStructSkelethalOrgan _mesh_8 (Utilities|Struct|MakeStructMeshParameters _material_8 _helmetcolor _parameters_3 false))) (Utilities|Array|MakeArray (Utilities|Struct|MakeStructStaticOrgan _mesh_2 (Utilities|Struct|MakeStructMeshParameters (Utilities|Array|MakeArray _material_2) (Utilities|Array|MakeArray _color) (Utilities|Array|MakeArray _parameter) false)) (Utilities|Struct|MakeStructStaticOrgan _mesh_3 (Utilities|Struct|MakeStructMeshParameters (Utilities|Array|MakeArray _material_3) _color_2 _parameter_2 false)))))

(fn ChestParameters
  (return (Utilities|Array|MakeArray "RedHsl" "GreenHSL" "BlueHSL" "BlackHSL")))

(fn CreateSword
  (bind _returnvalue (Math|Random|RandomIntegerinRange 0 10))
  (bind _weapons (Variables|CharacterCustomization|GetWeapons))
  (bind _returnvalue_2 (Utilities|Array|Length _weapons))
  (bind _returnvalue_3 (- _returnvalue_2 1))
  (bind _returnvalue_4 (Math|Random|RandomIntegerinRange 0 _returnvalue_3))
  (bind (_staticmesh _material) (Utilities|GetStaticMat _weapons _returnvalue_4 _returnvalue))
  (return _staticmesh _material (CallFunction|RandomSwordColor) "HSL"))

(fn RandomSwordColor
  (return (Utilities|MacRandomColor 0.0 1.0 0.0 1.0 0.0 1.0)))

(fn CreateShield
  (bind (_stroke _front _back _half) (CallFunction|RandomShieldColor))
  (bind _returnvalue (Math|Random|RandomIntegerinRange 0 10))
  (bind _returnvalue_2 (Math|Random|RandomIntegerinRange 0 10))
  (bind _shields (Variables|CharacterCustomization|GetShields))
  (bind _returnvalue_3 (Utilities|Array|Length _shields))
  (bind _returnvalue_4 (- _returnvalue_3 1))
  (bind _returnvalue_5 (Math|Random|RandomIntegerinRange 0 _returnvalue_4))
  (bind (_staticmesh _material) (Utilities|GetStaticMat _shields _returnvalue_5 _returnvalue_2 _returnvalue))
  (return _staticmesh _material (Utilities|Array|MakeArray _stroke _front _back _half) (Utilities|Array|MakeArray "RedHsl" "GreenHSL" "BlueHSL" "BlackHSL")))

(fn RandomShieldColor
  (bind _returnvalue (Utilities|MacRandomColor 0.0 2.0 0.0 1.3 0.0 1.3))
  (return _returnvalue _returnvalue _returnvalue _returnvalue))

(fn CreateRandomShoulder
  (bind _returnvalue (Math|Random|RandomIntegerinRange 0 10))
  (bind _returnvalue_2 (Math|Random|RandomIntegerinRange 0 10))
  (bind (_top _stroke _shoulder) (CallFunction|RandomShoulderColor))
  (bind _shoulders (Variables|CharacterCustomization|GetShoulders))
  (bind _returnvalue_3 (Utilities|GetRandomonLength _shoulders))
  (bind (_mesh _material) (Utilities|GetMeshMat _shoulders _returnvalue_3 _returnvalue_2 _returnvalue))
  (return _mesh (Utilities|Array|MakeArray _material) (Utilities|Array|MakeArray _top _stroke _shoulder) (Utilities|Array|MakeArray "RedHsl" "GreenHSL" "BlueHSL")))

(fn RandomShoulderColor
  (bind _returnvalue (Utilities|MacRandomColor 0.0 1.0 0.0 1.0 0.0 1.3))
  (return _returnvalue _returnvalue _returnvalue))

(fn CreateRandomGloves
  (bind _returnvalue (Math|Random|RandomIntegerinRange 0 4))
  (bind _returnvalue_2 (Math|Random|RandomIntegerinRange 0 4))
  (bind (_top _stroke _shoulder) (CallFunction|RandomShoulderColor))
  (bind _gloves (Variables|CharacterCustomization|GetGloves))
  (bind _returnvalue_3 (Utilities|GetRandomonLength _gloves))
  (bind (_mesh _material) (Utilities|GetMeshMat _gloves _returnvalue_3 _returnvalue_2 _returnvalue))
  (return _mesh (Utilities|Array|MakeArray _material) (Utilities|Array|MakeArray _top _stroke _shoulder) (Utilities|Array|MakeArray "RedHsl" "BlueHSL" "BlackHSL" "GreenHSL")))

(fn RandomGlovesColor
  (bind _returnvalue (Utilities|MacRandomColor 0.0 1.0 0.0 1.0 0.0 1.6))
  (return _returnvalue _returnvalue _returnvalue _returnvalue))

(fn CreateRandomHelmet
  (bind _returnvalue (Math|Random|RandomIntegerinRange 0 10))
  (bind _returnvalue_2 (Math|Random|RandomIntegerinRange 0 10))
  (bind _helmets (Variables|CharacterCustomization|GetHelmets))
  (bind _returnvalue_3 (Utilities|GetRandomonLength _helmets))
  (bind (_mesh _material) (Utilities|GetMeshMat _helmets _returnvalue_3 _returnvalue_2 _returnvalue))
  (return _mesh (Utilities|Array|MakeArray _material) (Utilities|Array|MakeArray (CallFunction|RandomHelmetColor)) (Utilities|Array|MakeArray "HSL")))

(fn RandomHelmetColor
  (return (Utilities|MacRandomColor 0.0 1.0 0.0 1.0 0.0 1.5)))