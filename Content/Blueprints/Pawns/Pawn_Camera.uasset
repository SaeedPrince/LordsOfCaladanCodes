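; Camera pawn with a Move event that shifts it along a Forward or Right direction relative to its own rotation.
; Move derives the direction from a Z-based rotator via GetMovementVector, then applies movement input scaled by the axis value and MoveTile, with the sign inverted.
; It also prints that vector for debugging.
; A local GetVector helper maps Direction to forward or right vectors, but Move does not call it.
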(event Custom|Move
  (params (AxisValue :type Float%20%28single-precision%29) (Direction :type String))
  (bind _returnvalue (Transformation|GetActorRotation))
  (bind _returnvalue_2 (Class|LordsOfCaladanFunctionLibrary|MakeRotatorbyZ _returnvalue))
  (bind _returnvalue_3 (Class|LordsOfCaladanFunctionLibrary|GetMovementVector _returnvalue_2 Direction))
  ;[1 1 0] Movement
  (Pawn|Input|AddMovementInput _returnvalue_3 (* AxisValue (Variables|Customization|GetMoveTile) -1.0) false)
  (Development|PrintString (Utilities|String|ToString(Vector) _returnvalue_3)))

(fn ConstructionScript)

(fn GetVector
  (params (Rotator :type Rotator) (Direction :type String))
  (switch string Direction
    (:Forward
      (LocalVariables|SetOutVector (Math|Vector|GetForwardVector Rotator)))
    (:Right
      (LocalVariables|SetOutVector (Math|Vector|GetRightVector Rotator))))
  (return (LocalVariables|GetOutVector)))