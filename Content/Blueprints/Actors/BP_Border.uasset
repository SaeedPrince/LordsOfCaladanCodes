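; BP_Border is a border actor whose construction script tints BorderComponent00 green through its GlassColor parameter.
; Its event graph holds only disabled placeholder events, so it has no runtime behavior of its own.
; ActorIsInside appears meant to test an actor's bounds against the child components, but it is unfinished: the loop body is empty, the bounds math is unused and the return node is never reached.
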(event EventBeginPlay)

(event Collision|EventActorBeginOverlap
  (params (OtherActor :type Actor%20Object%20Reference)))

(event EventTick
  (params (DeltaSeconds :type Float%20%28single-precision%29)))

(fn ConstructionScript
  (CallFunction|SetComponentColor (Variables|Default|GetBorderComponent00) "GlassColor" "Green"))

(fn ActorIsInside
  (params (ActorOrigin :type Vector) (ActorBoxExtent :type Vector))
  (bind _array_element (Utilities|Array|ForEachLoopwithBreak (Components|GetChildrenComponents (Variables|Default|GetDefaultSceneRoot) false))))