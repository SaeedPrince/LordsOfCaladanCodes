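; BP_Box is a box actor with a tinted glass mesh that can report whether another actor's bounds lie inside it.
; BeginPlay applies the Color variable to the GlassColor parameter on BoxMesh.
; ActorIsInside tests the supplied origin and extent against the bounds of each direct child of DefaultSceneRoot using BoxIsInsideBox, returning true at the first containing component.
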(event EventBeginPlay
  (CallFunction|SetComponentColorbyLinearColor (Variables|Default|GetBoxMesh) "GlassColor" (Variables|SpawnData|GetColor)))

(fn ConstructionScript)

(fn ActorIsInside
  (params (ActorOrigin :type Vector) (ActorBoxExtent :type Vector))
  (bind _array_element (Utilities|Array|ForEachLoopwithBreak (Components|GetChildrenComponents (Variables|Default|GetDefaultSceneRoot) false) :!label _label)
    (:LoopBody
      (if (CallFunction|BoxIsInsideBox (.Origin (Collision|GetComponentBounds _array_element)) (.BoxExtent (Collision|GetComponentBounds _array_element)) ActorOrigin ActorBoxExtent)
        (LocalVariables|SetOutBool true)
        (goto _label Break)))
    (:Completed
      (return (LocalVariables|GetOutBool)))))