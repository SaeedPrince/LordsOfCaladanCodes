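; Blueprint function library of color helpers for tinting components by color name.
; GetColorByString maps six names of primary and secondary colors to opaque linear colors.
; SetComponentColor creates a dynamic material instance on a primitive component's first material slot and writes that color to a named vector parameter.
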(fn GetColorbyString
  (params (Color :type String))
  (switch string Color
    (:Red
      (LocalVariables|SetOutColor (Utilities|Struct|MakeLinearColor 1.0 0.0 0.0 1.0)))
    (:Green
      (LocalVariables|SetOutColor (Utilities|Struct|MakeLinearColor 0.0 1.0 0.0 1.0)))
    (:Blue
      (LocalVariables|SetOutColor (Utilities|Struct|MakeLinearColor 0.0 0.0 1.0 1.0)))
    (:Yellow
      (LocalVariables|SetOutColor (Utilities|Struct|MakeLinearColor 1.0 1.0 0.0 1.0)))
    (:Cyan
      (LocalVariables|SetOutColor (Utilities|Struct|MakeLinearColor 0.0 1.0 1.0 1.0)))
    (:Purple
      (LocalVariables|SetOutColor (Utilities|Struct|MakeLinearColor 1.0 0.0 1.0 1.0))))
  (return (LocalVariables|GetOutColor)))

(fn SetComponentColor
  (params (PrimitiveComponent :type Primitive%20Component%20Object%20Reference) (Parameter :type Name) (Color :type String))
  (bind _returnvalue (Rendering|Material|CreateDynamicMaterialInstance PrimitiveComponent 0 0 :!class /Script/Engine.PrimitiveComponent))
  (Rendering|Material|SetVectorParameterValue _returnvalue Parameter (CallFunction|GetColorbyString Color) :!class /Script/Engine.MaterialInstanceDynamic))