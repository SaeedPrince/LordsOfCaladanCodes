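; AI controller for a civilian person who lives in one building and can work and carry items for others.
; The construction script takes character, residence and placement from spawn data, then starts the civilian behavior tree and seeds its blackboard.
; Server events track home and work presence, notify the workplace, and attach, drop or destroy inventory items, informing buildings on pickup and drop.
; A position change refreshes the owning player's bottom widget.
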(event Custom|ServerPersonIsAtWork
  (bind _buildingwork (Variables|Building|GetBuildingWork))
  ;[1 1 0] Building start to work or stop
  (Utilities|IsValid _buildingwork
    (:Is%20Valid
      (Default|ServerWorkerArrivedWork _buildingwork (Variables|Data|GetType) (Variables|Building|GetIndexInWorker)))))

(event Custom|ServerPersonLeftWork
  (bind _buildingwork (Variables|Building|GetBuildingWork))
  ;[1 1 0] Building start to work or stop
  (Variables|Data|SetIsAtWork false)
  (Utilities|IsValid _buildingwork
    (:Is%20Valid
      (Default|ServerWorkerLeftWork _buildingwork (Variables|Data|GetType) (Variables|Building|GetIndexInWorker)))))

(event Custom|ServerPickupItem
  (params (Item :type BP%20Item%20Object%20Reference) (Building :type BP%20House%20Object%20Reference))
  ;[1 1 0] Career item pickup or drop
  (Utilities|Array|Add (Variables|Item|GetInventory) Item)
  (Transformation|AttachActorToActor Item (Variables|GameObject|GetCharacterRef) "hand_rSocket" "SnapToTarget" "SnapToTarget" "SnapToTarget" false)
  (Default|ServerItemSent Building Item))

(event Custom|ServerDropItem
  (params (Item :type BP%20Item%20Object%20Reference) (Building :type BP%20House%20Object%20Reference))
  ;[1 1 0] Career item pickup or drop
  (Utilities|MacRemoveItem Item)
  (Default|ServerItemReceived Building Item))

(event Custom|ServerPersonLeftHome
  ;[1 1 0] Building start to work or stop
  (Variables|Data|SetIsAtHome false))

(event Custom|PersonPositionChanged
  (bind _buildingresidence (Variables|Building|GetBuildingResidence))
  (bind _player (Variables|/Game/Assets/BP_Meshes/Architecture/BP_House.BP_House_C|GetPlayer _buildingresidence))
  ;[0 1 0] Updates bottom widget
  (if (Variables|/Game/Blueprints/Controllers/PlayerController_Game.PlayerController_Game_C|GetBottomWidget _player)
    (Default|ShowBottomData _player)))

(event Custom|ServerPersonIsAtHome
  ;[1 1 0] Building start to work or stop
  (Variables|Data|SetIsAtHome true))

(event Custom|ServerWasteItem
  (params (Item :type BP%20Item%20Object%20Reference))
  ;[1 1 0] Career item pickup or drop
  (Utilities|MacRemoveItem Item)
  (Actor|DestroyActor Item))

(fn ConstructionScript
  (bind _self self)
  (bind _spawndata (Variables|GameObject|GetSpawnData))
  (bind (_characterref _building _placement) (Utilities|Struct|BreakStructAI _spawndata))
  (bind _returnvalue (AI|GetBlackboard _self))
  (Variables|GameObject|SetCharacterRef _characterref)
  (Variables|Building|SetBuildingResidence _building)
  (Variables|Placements|SetResidentPlacement _placement)
  (Variables|GameObject|SetCurrentBlackBoard "/Game/Blueprints/AI/BehaviorTree/BB_Human.BB_Human")
  (Variables|GameObject|SetCurrentBehaviorTree "/Game/Blueprints/AI/BehaviorTree/BT_Civilian.BT_Civilian")
  (Class|AIController|UseBlackboard (Variables|GameObject|GetCurrentBlackBoard))
  (AI|RunBehaviorTree (Variables|GameObject|GetCurrentBehaviorTree))
  (AI|Components|Blackboard|SetValueasVector _returnvalue (Variables|Blackboard|GetHomeLocation) (Variables|Placements|GetResidentPlacement))
  (AI|Components|Blackboard|SetValueasObject _returnvalue (Variables|Blackboard|GetSelfActor) (Variables|GameObject|GetCharacterRef)))

(fn BuildingRefbyPerson
  (return (.Building (Utilities|Struct|BreakStructAI (Variables|GameObject|GetSpawnData))) (Variables|Data|GetType) (.PersonIndex (Utilities|Struct|BreakStructPersonSpawnResult (Variables|GameObject|GetSpawnResult)))))