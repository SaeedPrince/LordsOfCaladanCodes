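; Player controller for the front-end menus, opening the game setup screen on begin play for clients and non-dedicated servers.
; Events show the join server, create character, game setup and load character screens, refreshing or clearing some on display.
; A shared macro swaps the current widget, creating each lazily with a back-reference to the controller and caching it in an array by index for reuse.
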(event Custom|ShowJoinServerMenu
  ;[1 1 0] Show join server menu
  (Utilities|MacShowWidget (Variables|Widget|GetWidgetClient) "/Game/Blueprints/Widgets/Widget_Client.Widget_Client_C"))

(event Custom|ShowCreateCharacterMenu
  ;[1 1 0] Show create character menu
  (Utilities|MacShowWidget (Variables|Widget|GetWidgetCreateCharacter) "/Game/Blueprints/Widgets/Widget_CharacterSetup.Widget_CharacterSetup_C")
  (bind _aswidget_character_setup (Utilities|Casting|CastToWidget_CharacterSetup (Variables|Widget|GetCurrentWidget)))
  (Default|ClearPage _aswidget_character_setup))

(event Custom|ShowGameSetupMenu
  (params (CheckForCharacterNumber :type Boolean) (CharacterSelected :type Boolean) (SelectedCharacter :type Struct%20Character%20Structure))
  ;[1 1 0] Show game setup menu
  (Utilities|MacShowWidget (Variables|Widget|GetWidgetGameSetup) "/Game/Blueprints/Widgets/Widget_GameSetup.Widget_GameSetup_C")
  (if CheckForCharacterNumber
    (bind _aswidget_game_setup (Utilities|Casting|CastToWidget_GameSetup (Variables|Widget|GetCurrentWidget)))
    (Default|CheckforCharacterNum _aswidget_game_setup CharacterSelected SelectedCharacter)))

(event Custom|ShowLoadCharacterMenu
  ;[1 1 0] Show load character menu
  (Utilities|MacShowWidget (Variables|Widget|GetWidgetLoadCharacter) "/Game/Blueprints/Widgets/Widget_CharacterLoad.Widget_CharacterLoad_C")
  (bind _aswidget_character_load (Utilities|Casting|CastToWidget_CharacterLoad (Variables|Widget|GetCurrentWidget)))
  (Default|UpdateWidget _aswidget_character_load))

(event EventBeginPlay
  ;[1 1 0] Begin play
  (Networking|SwitchHasAuthority
    (:Authority
      (if (not (Networking|IsDedicatedServer))
        (CallFunction|ShowGameSetupMenu false false :!label _label)))
    (:Remote
      (goto _label))))

(fn ConstructionScript)