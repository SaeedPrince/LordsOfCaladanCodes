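; Player controller for a multiplayer game that handles character input and each player's path from joining to spawning a MedievalWarrior.
; Input drives appearance changes, attack poses and movement or camera control, switching on FPS, RTS or TPS camera mode.
; Server events use GameMode state to cap players, queue color picking one at a time, and hold lobby entry behind it.
; Lobby updates and readiness fan out to all controllers' widgets, while joining can bypass the lobby with random attributes.
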(event Input|ActionEvents|InputActionDefend-MoveToPoint-Navigation
  (params (Key :type Key%20Structure))
  ;[1 1 0] Defend - Move to point - Camera navigation enable
  (:Pressed
    (Variables|State|SetIsPressingRightMouse true))
  (:Released
    (Variables|State|SetIsPressingRightMouse false)))

(event Input|ActionEvents|InputActionChangeFace
  (params (Key :type Key%20Structure))
  ;[1 1 0] Change apearance
  (:Pressed
    (Default|SetFace (Variables|GameObject|GetCharacterRef))))

(event Input|ActionEvents|InputActionChangeShild
  (params (Key :type Key%20Structure))
  ;[1 1 0] Change apearance
  (:Pressed
    (Default|SetShield (Variables|GameObject|GetCharacterRef) false)))

(event Input|ActionEvents|InputActionChangeWeapon
  (params (Key :type Key%20Structure))
  ;[1 1 0] Change apearance
  (:Pressed
    (Default|SetWeapon (Variables|GameObject|GetCharacterRef) false)))

(event Input|ActionEvents|InputActionChangeShoulder
  (params (Key :type Key%20Structure))
  ;[1 1 0] Change apearance
  (:Pressed
    (Default|SetShoulder (Variables|GameObject|GetCharacterRef) false)))

(event Input|ActionEvents|InputActionChangeCamera
  (params (Key :type Key%20Structure))
  (bind _characterref (Variables|GameObject|GetCharacterRef))
  (bind _fpscamera (Variables|/Game/Blueprints/Characters/MedievalWarrior.MedievalWarrior_C|GetFPSCamera _characterref))
  (bind _tpscamera (Variables|/Game/Blueprints/Characters/MedievalWarrior.MedievalWarrior_C|GetTPSCamera _characterref))
  (bind _rtscamera (Variables|/Game/Blueprints/Characters/MedievalWarrior.MedievalWarrior_C|GetRTSCamera _characterref))
  ;[1 1 0] Change Camera
  (:Pressed
    (switch int (Variables|Camera|GetCurrentCamera) ; FPS=1, RTS=2, TPS=3
      (:1
        (Components|Activation|Deactivate _fpscamera)
        (Components|Activation|Activate _rtscamera false)
        (Variables|Camera|SetCurrentCamera (Variables|DefaultValue|GetRTS))
        (Variables|Default|SetbShowMouseCursor true))
      (:2
        (Components|Activation|Deactivate _rtscamera)
        (Components|Activation|Activate _tpscamera false)
        (Variables|Camera|SetCurrentCamera (Variables|DefaultValue|GetTPS))
        (Variables|Default|SetbShowMouseCursor false))
      (:3
        (Components|Activation|Deactivate _tpscamera)
        (Components|Activation|Activate _fpscamera false)
        (Variables|Camera|SetCurrentCamera (Variables|DefaultValue|GetFPS))))))

(event Input|ActionEvents|InputActionChangeChest
  (params (Key :type Key%20Structure))
  ;[1 1 0] Change apearance
  (:Pressed
    (Default|SetChest (Variables|GameObject|GetCharacterRef))))

(event Input|ActionEvents|InputActionChangeGloves
  (params (Key :type Key%20Structure))
  ;[1 1 0] Change apearance
  (:Pressed
    (Default|SetGloves (Variables|GameObject|GetCharacterRef) false)))

(event Input|ActionEvents|InputActionChangeBoots
  (params (Key :type Key%20Structure))
  ;[1 1 0] Change apearance
  (:Pressed
    (Default|SetBoots (Variables|GameObject|GetCharacterRef))))

(event Input|ActionEvents|InputActionChangePants
  (params (Key :type Key%20Structure))
  ;[1 1 0] Change apearance
  (:Pressed
    (Default|SetPants (Variables|GameObject|GetCharacterRef))))

(event Input|ActionEvents|InputActionAttack-Select
  (params (Key :type Key%20Structure))
  (bind _characterref (Variables|GameObject|GetCharacterRef))
  (bind _isattacking (Variables|/Game/Blueprints/Characters/FighterBP.FighterBP_C|GetIsAttacking _characterref))
  ;[1 1 0] Attack - Select
  (:Pressed
    (Variables|State|SetIsPressingLeftMouse true)
    (Utilities|IsValid _characterref
      (:Is%20Valid
        (if (not _isattacking)
          (Default|PlayerAttackPoseStart _characterref)))))
  (:Released
    (Variables|State|SetIsPressingLeftMouse false)
    (Utilities|IsValid _characterref
      (:Is%20Valid
        (if _isattacking
          (Default|PlayerAttackPoseEnd _characterref))))))

(event Input|ActionEvents|InputActionChangeHood
  (params (Key :type Key%20Structure))
  ;[1 1 0] Change apearance
  (:Pressed
    (Default|SetHood (Variables|GameObject|GetCharacterRef) false)))

(event Input|ActionEvents|InputActionChangeHair
  (params (Key :type Key%20Structure))
  ;[1 1 0] Change apearance
  (:Pressed
    (Default|SetHair (Variables|GameObject|GetCharacterRef) false)))

(event Input|ActionEvents|InputActionChangeHelmet
  (params (Key :type Key%20Structure))
  ;[1 1 0] Change apearance
  (:Pressed
    (Default|SetHelmet (Variables|GameObject|GetCharacterRef) false)))

(event Input|AxisEvents|InputAxisTurn
  (params (AxisValue :type Float%20%28single-precision%29))
  (bind _characterref (Variables|GameObject|GetCharacterRef))
  ;[1 1 0] Mouse Movement
  (if (!= AxisValue 0.0)
    (Utilities|IsValid _characterref
      (:Is%20Valid
        (switch int (Variables|Camera|GetCurrentCamera) ; FPS=1, RTS=2, TPS=3
          (:1
            (Default|TurnPlayer _characterref AxisValue :!label _label))
          (:2
            (if (Variables|State|GetIsPressingRightMouse)
              (Default|RTSCameraRotateZ _characterref AxisValue)))
          (:3
            (goto _label)))))))

(event Input|AxisEvents|InputAxisMoveForward
  (params (AxisValue :type Float%20%28single-precision%29))
  (bind _characterref (Variables|GameObject|GetCharacterRef))
  ;[1 1 0] Character movement, Camera movement
  (if (!= AxisValue 0.0)
    (switch int (Variables|Camera|GetCurrentCamera) ; FPS=1, RTS=2, TPS=3
      (:1
        (Default|PlayerMove _characterref AxisValue "Forward" :!label _label))
      (:2
        (if (Variables|State|GetIsPressingRightMouse)
          (Default|RTSCameraMoveForward _characterref AxisValue)))
      (:3
        (goto _label)))))

(event Input|AxisEvents|InputAxisMoveRight
  (params (AxisValue :type Float%20%28single-precision%29))
  (bind _characterref (Variables|GameObject|GetCharacterRef))
  ;[1 1 0] Character movement, Camera movement
  (if (!= AxisValue 0.0)
    (switch int (Variables|Camera|GetCurrentCamera) ; FPS=1, RTS=2, TPS=3
      (:1
        (Default|PlayerMove _characterref AxisValue "Right" :!label _label))
      (:2
        (if (Variables|State|GetIsPressingRightMouse)
          (Default|RTSCameraMoveRight _characterref AxisValue)))
      (:3
        (goto _label)))))

(event Input|AxisEvents|InputAxisCameraZoom
  (params (AxisValue :type Float%20%28single-precision%29))
  ;[1 1 0] Camera Zoom
  (if (!= AxisValue 0.0)
    (switch int (Variables|Camera|GetCurrentCamera) ; FPS=1, RTS=2, TPS=3
      (:2
        (Default|RTSCameraMoveForward (Variables|GameObject|GetCharacterRef) AxisValue)))))

(event Input|AxisEvents|InputAxisLookUp
  (params (AxisValue :type Float%20%28single-precision%29))
  (bind _characterref (Variables|GameObject|GetCharacterRef))
  ;[1 1 0] Mouse Movement
  (if (!= AxisValue 0.0)
    (Utilities|IsValid _characterref
      (:Is%20Valid
        (switch int (Variables|Camera|GetCurrentCamera) ; FPS=1, RTS=2, TPS=3
          (:1
            (Default|LookupPlayer _characterref AxisValue :!label _label))
          (:2
            (if (Variables|State|GetIsPressingRightMouse)
              (Default|RTSCameraRotateY _characterref AxisValue)))
          (:3
            (goto _label)))))))

(event Custom|ServerSpawnPlayer
  (params (PlayerColor :type Linear%20Color%20Structure) (SpawnPlace :type Integer))
  ;[1 1 0] Spawn Player
  (Default|CreateNewCharacter (Variables|GameObject|GetGameModeRef) "/Game/Blueprints/Characters/MedievalWarrior.MedievalWarrior_C" self PlayerColor SpawnPlace))

(event Custom|StopGameCountDown
  ;[1 1 0] Lobby
  (Default|StopGameStartTimer (Variables|Widget|GetWidgetLobbyRef)))

(event Custom|WaitForLobby
  ;[1 1 0] Lobby
  (bind _widgetshown (Utilities|MacCreateWidget true "/Game/Blueprints/Widgets/Wait.Wait_C"))
  (bind _aswait (Utilities|Casting|CastToWait _widgetshown))
  (bind _output_get (Variables|Widget|SetWidgetWaitRef _aswait))
  (Default|StartWaitforLobby _output_get self))

(event Custom|ServerColorPickedAndNameTaken
  (bind _gamemoderef (Variables|GameObject|GetGameModeRef))
  ;[1 1 0] After pick color and name taken
  (if (or (Variables|/Game/Blueprints/GameModes/GameMode_Game.GameMode_Game_C|GetSomeoneIsPickingColor _gamemoderef) (> (Variables|/Game/Blueprints/GameModes/GameMode_Game.GameMode_Game_C|GetWaitingForPickColor _gamemoderef) 0))
    (Variables|/Game/Blueprints/GameModes/GameMode_Game.GameMode_Game_C|SetWaitingForLobby _gamemoderef (+ (Variables|/Game/Blueprints/GameModes/GameMode_Game.GameMode_Game_C|GetWaitingForLobby _gamemoderef) 1))
    (CallFunction|WaitforLobby)
    (else
      (CallFunction|JoinLobby))))

(event Custom|JoinLobby
  ;[1 1 0] Lobby
  (bind _returnvalue (UserInterface|CreateWidget "/Game/Blueprints/Widgets/Lobby.Lobby_C" self))
  (bind _output_get (Variables|Widget|SetWidgetLobbyRef _returnvalue))
  (UserInterface|Viewport|AddtoViewport _output_get 0)
  (Variables|/Game/Blueprints/Widgets/Lobby.Lobby_C|SetPlayerColor _returnvalue (Variables|Player|GetPlayerColor))
  (Variables|/Game/Blueprints/Widgets/Lobby.Lobby_C|SetPlayerName _returnvalue (Variables|Player|GetUsername))
  (Default|InitialLobby _returnvalue self)
  (Variables|State|SetIsAtLobby true)
  (CallFunction|ServerInitiateLobbyData (Variables|Player|GetPlayerColor) (Variables|Player|GetUsername)))

(event Custom|StopWaitForLobby
  (bind _widgetwaitref (Variables|Widget|GetWidgetWaitRef))
  ;[1 1 0] Stop Wait for lobby
  (Default|StopWaitforLobby _widgetwaitref)
  (Widget|RemovefromParent _widgetwaitref))

(event Custom|ClientColorPicked
  (params (PlayerColor :type Linear%20Color%20Structure))
  (bind _self self)
  ;[0 1 0] Pick player color
  (Variables|Player|SetPlayerColor PlayerColor)
  (if (Utilities|Enum|Equal(Enum) (Variables|Player|GetUsername) (Utilities|Text|MakeLiteralText ""))
    (CallFunction|ServerRequestRandomName _self))
  (CallFunction|ServerColorPickedandNameTaken _self))

(event Custom|ServerColorPicked
  (params (ColorPicked :type Linear%20Color%20Structure))
  (bind _gamemoderef (Variables|GameObject|GetGameModeRef))
  ;[1 1 0] Color picked
  (Variables|/Game/Blueprints/GameModes/GameMode_Game.GameMode_Game_C|SetSomeoneIsPickingColor _gamemoderef false)
  (Utilities|Array|RemoveItem (Variables|/Game/Blueprints/GameModes/GameMode_Game.GameMode_Game_C|GetAvailableColors _gamemoderef) ColorPicked))

(event Custom|ServerInitiateLobbyData
  (params (PlayerColor :type Linear%20Color%20Structure) (PlayerName :type Text))
  (bind _gamemoderef (Variables|GameObject|GetGameModeRef))
  ;[1 1 0] Lobby
  (Utilities|Array|AddUnique (Variables|/Game/Blueprints/GameModes/GameMode_Game.GameMode_Game_C|GetLobbyPlayerColors _gamemoderef) PlayerColor)
  (Utilities|Array|AddUnique (Variables|/Game/Blueprints/GameModes/GameMode_Game.GameMode_Game_C|GetLobbyPlayerNames _gamemoderef) PlayerName)
  (CallFunction|ServerUpdateLobbyforAll))

(event Custom|StopWaitForPickColor
  (bind _widgetwaitref (Variables|Widget|GetWidgetWaitRef))
  ;[1 1 0] Stop waiting for pick color
  (Default|StopWaitforPickColor _widgetwaitref)
  (Widget|RemovefromParent _widgetwaitref))

(event Custom|ServerUpdateLobbyForAll
  (bind _gamemoderef (Variables|GameObject|GetGameModeRef))
  ;[1 1 0] Lobby
  (bind _outactors (Actor|GetAllActorsOfClass "PlayerController_Game_C"))
  (for _array_element _outactors
    (CallFunction|UpdateLobby _array_element (Variables|/Game/Blueprints/GameModes/GameMode_Game.GameMode_Game_C|GetLobbyPlayerNames _gamemoderef) (Variables|/Game/Blueprints/GameModes/GameMode_Game.GameMode_Game_C|GetGamePlayerNames _gamemoderef) (Variables|/Game/Blueprints/GameModes/GameMode_Game.GameMode_Game_C|GetLobbyPlayerColors _gamemoderef) (Variables|/Game/Blueprints/GameModes/GameMode_Game.GameMode_Game_C|GetGamePlayerColors _gamemoderef) (Variables|/Game/Blueprints/GameModes/GameMode_Game.GameMode_Game_C|GetGameReadyVisible _gamemoderef))))

(event Custom|ServerRequestForPickColor
  (bind _gamemoderef (Variables|GameObject|GetGameModeRef))
  ;[1 1 0] Request for pick color
  (if (Variables|/Game/Blueprints/GameModes/GameMode_Game.GameMode_Game_C|GetSomeoneIsPickingColor _gamemoderef)
    (CallFunction|ShowStatsonWait (Utilities|Text|ToText(Integer) (Variables|/Game/Blueprints/GameModes/GameMode_Game.GameMode_Game_C|GetWaitingForPickColor _gamemoderef)) (Utilities|Text|ToText(Integer) (Variables|/Game/Blueprints/GameModes/GameMode_Game.GameMode_Game_C|GetWaitingForLobby _gamemoderef)))
    (else
      (CallFunction|StopWaitforPickColor)
      (Variables|/Game/Blueprints/GameModes/GameMode_Game.GameMode_Game_C|SetSomeoneIsPickingColor _gamemoderef true)
      (Variables|/Game/Blueprints/GameModes/GameMode_Game.GameMode_Game_C|SetWaitingForPickColor _gamemoderef (- (Variables|/Game/Blueprints/GameModes/GameMode_Game.GameMode_Game_C|GetWaitingForPickColor _gamemoderef) 1))
      (CallFunction|PickPlayerColor (Variables|/Game/Blueprints/GameModes/GameMode_Game.GameMode_Game_C|GetAvailableColors _gamemoderef)))))

(event Custom|RequestSpawnPlayer
  (params (SpawnPlace :type Integer))
  ;[1 1 0] Spawn Player
  (Variables|Default|SetbShowMouseCursor false)
  (Widget|RemovefromParent (Variables|Widget|GetWidgetLobbyRef))
  (CallFunction|ServerSpawnPlayer (Variables|Player|GetPlayerColor) SpawnPlace))

(event Custom|ShowStatsOnWait
  (params (Pick :type Text) (Lobby :type Text))
  ;[1 1 0] Show stats when waiting
  (Default|ShowStats (Variables|Widget|GetWidgetWaitRef) Pick Lobby))

(event Custom|SaveAttributes
  (params (Username :type Text) (Color :type Linear%20Color%20Structure))
  ;[0 1 0] Save Username
  (Variables|Player|SetUsername Username)
  (Variables|Player|SetPlayerColor Color)
  (Variables|Player|SetRandomAttributes true)
  (Variables|Default|SetbShowMouseCursor false))

(event Custom|QuitBecauseNotReady
  ;[0 1 0] Quit if more than max player or not ready
  (Development|PrintString "Game started and you were not ready." true true "(R=1.000000,G=0.000000,B=0.000000,A=1.000000)" 1e+01)
  (Utilities|FlowControl|Delay 1e+01)
  (Game|QuitGame self "Quit"))

(event Custom|ServerUpdateReadiness
  (params (Readiness :type Array%20of%20Booleans))
  (bind _gamemoderef (Variables|GameObject|GetGameModeRef))
  ;[1 1 0] Lobby
  (Variables|/Game/Blueprints/GameModes/GameMode_Game.GameMode_Game_C|SetGameReadyChecked _gamemoderef Readiness)
  (bind _outactors (Actor|GetAllActorsOfClass "PlayerController_Game_C"))
  (for _array_element _outactors
    (CallFunction|UpdateReadiness _array_element (Variables|/Game/Blueprints/GameModes/GameMode_Game.GameMode_Game_C|GetGameReadyChecked _gamemoderef))
    (if (Default|ReadytoStart _gamemoderef)
      (CallFunction|StartGameCountDown _array_element)
      (else
        (CallFunction|StopGameCountDown _array_element)))))

(event Custom|ServerRequestJoinNewPlayer
  (params (Username :type Text) (BypassLobby :type Boolean))
  ;[0 1 0] Request to join happens on the server
  (bind _instanceref (Utilities|MacGetGameInstance))
  (bind _gamemoderef (Utilities|MacGetGameMode))
  (if (< (Variables|/Game/Blueprints/GameModes/GameMode_Game.GameMode_Game_C|GetConnectedPlayers _gamemoderef) (Variables|/Game/Blueprints/GameInstances/TheInstance.TheInstance_C|GetMaxClient _instanceref))
    (Variables|/Game/Blueprints/GameModes/GameMode_Game.GameMode_Game_C|SetConnectedPlayers _gamemoderef (+ (Variables|/Game/Blueprints/GameModes/GameMode_Game.GameMode_Game_C|GetConnectedPlayers _gamemoderef) 1))
    (if (Utilities|Enum|Equal(Enum) Username (Utilities|Text|MakeLiteralText ""))
      _
      (else
        (CallFunction|SaveUsername Username false)))
    (if BypassLobby
      (bind _rndusername (Default|GetRandomUsername _gamemoderef))
      (bind _rndcolor (Default|GetRandomPlayerColor _gamemoderef))
      (bind _spawnplace (Default|GetSpawnPlacebyOrder _gamemoderef))
      (CallFunction|SaveAttributes _rndusername _rndcolor)
      (Default|CreateNewCharacter _gamemoderef "/Game/Blueprints/Characters/MedievalWarrior.MedievalWarrior_C" self _rndcolor _spawnplace)
      (elif (Variables|/Game/Blueprints/GameModes/GameMode_Game.GameMode_Game_C|GetSomeoneIsPickingColor _gamemoderef)
        (Variables|/Game/Blueprints/GameModes/GameMode_Game.GameMode_Game_C|SetWaitingForPickColor _gamemoderef (+ (Variables|/Game/Blueprints/GameModes/GameMode_Game.GameMode_Game_C|GetWaitingForPickColor _gamemoderef) 1))
        (CallFunction|WaitforPickColor)
        (else
          (Variables|/Game/Blueprints/GameModes/GameMode_Game.GameMode_Game_C|SetSomeoneIsPickingColor _gamemoderef true)
          (CallFunction|PickPlayerColor (Variables|/Game/Blueprints/GameModes/GameMode_Game.GameMode_Game_C|GetAvailableColors _gamemoderef)))))
    (else
      (CallFunction|NoMorePlayerAllowed))))

(event Custom|UpdateReadiness
  (params (Readiness :type Array%20of%20Booleans))
  (bind _widgetlobbyref (Variables|Widget|GetWidgetLobbyRef))
  ;[1 1 0] Lobby
  (Variables|/Game/Blueprints/Widgets/Lobby.Lobby_C|SetGameReadyChecked _widgetlobbyref Readiness)
  (Default|ArrangeReadiness _widgetlobbyref))

(event Custom|ServerPlayerQuit
  (bind _gamemoderef (Variables|GameObject|GetGameModeRef))
  ;[1 1 0] Add to available colors in case of quit player
  (Utilities|Array|AddUnique (Variables|/Game/Blueprints/GameModes/GameMode_Game.GameMode_Game_C|GetAvailableColors _gamemoderef) (Variables|Player|GetPlayerColor))
  (Variables|/Game/Blueprints/GameModes/GameMode_Game.GameMode_Game_C|SetConnectedPlayers _gamemoderef (- (Variables|/Game/Blueprints/GameModes/GameMode_Game.GameMode_Game_C|GetConnectedPlayers _gamemoderef) 1)))

(event Custom|SaveUsername
  (params (Username :type Text) (rndUsername :type Boolean))
  ;[0 1 0] Save Username
  (Variables|Player|SetUsername Username)
  (Variables|Player|SetRandomAttributes rndUsername))

(event Custom|UpdateLobby
  (params (LobbyNames :type Array%20of%20Texts) (GameNames :type Array%20of%20Texts) (LobbyColors :type Array%20of%20Linear%20Color%20Structures) (GameColors :type Array%20of%20Linear%20Color%20Structures) (ReadyVisible :type Array%20of%20Booleans))
  (bind _widgetlobbyref (Variables|Widget|GetWidgetLobbyRef))
  ;[1 1 0] Lobby
  (Variables|/Game/Blueprints/Widgets/Lobby.Lobby_C|SetLobbyPlayerNames _widgetlobbyref LobbyNames)
  (Variables|/Game/Blueprints/Widgets/Lobby.Lobby_C|SetLobbyPlayerColors _widgetlobbyref LobbyColors)
  (Variables|/Game/Blueprints/Widgets/Lobby.Lobby_C|SetGamePlayerNames _widgetlobbyref GameNames)
  (Variables|/Game/Blueprints/Widgets/Lobby.Lobby_C|SetGamePlayerColors _widgetlobbyref GameColors)
  (Variables|/Game/Blueprints/Widgets/Lobby.Lobby_C|SetGameReadyVisible _widgetlobbyref ReadyVisible)
  (Default|ArrangeLobby _widgetlobbyref))

(event Custom|ServerRequestForJoinLobby
  (bind _gamemoderef (Variables|GameObject|GetGameModeRef))
  ;[1 1 0] Lobby
  (if (or (Variables|/Game/Blueprints/GameModes/GameMode_Game.GameMode_Game_C|GetSomeoneIsPickingColor _gamemoderef) (> (Variables|/Game/Blueprints/GameModes/GameMode_Game.GameMode_Game_C|GetWaitingForPickColor _gamemoderef) 0))
    (CallFunction|ShowStatsonWait (Utilities|Text|ToText(Integer) (Variables|/Game/Blueprints/GameModes/GameMode_Game.GameMode_Game_C|GetWaitingForPickColor _gamemoderef)) (Utilities|Text|ToText(Integer) (Variables|/Game/Blueprints/GameModes/GameMode_Game.GameMode_Game_C|GetWaitingForLobby _gamemoderef)))
    (else
      (bind _outactors (Actor|GetAllActorsOfClass "PlayerController_Game_C"))
      (for _array_element _outactors
        (if (and (not (Variables|PlayerController_Game_C|GetIsAtLobby _array_element)) (not (Variables|PlayerController_Game_C|GetIsAtGame _array_element)))
          (CallFunction|StopWaitforLobby _array_element)
          (Variables|/Game/Blueprints/GameModes/GameMode_Game.GameMode_Game_C|SetWaitingForLobby _gamemoderef (- (Variables|/Game/Blueprints/GameModes/GameMode_Game.GameMode_Game_C|GetWaitingForLobby _gamemoderef) 1))
          (CallFunction|JoinLobby _array_element))))))

(event Custom|NoMorePlayerAllowed
  ;[0 1 0] Quit if more than max player or not ready
  (Development|PrintString "No more player allowed." true true "(R=1.000000,G=0.000000,B=0.000000,A=1.000000)" 1e+01)
  (Utilities|FlowControl|Delay 1e+01)
  (Game|QuitGame self "Quit"))

(event Custom|ServerUpdateLobbyData
  (params (LobbyNames :type Array%20of%20Texts) (GameNames :type Array%20of%20Texts) (LobbyColors :type Array%20of%20Linear%20Color%20Structures) (GameColors :type Array%20of%20Linear%20Color%20Structures) (ReadyVisible :type Array%20of%20Booleans))
  (bind _gamemoderef (Variables|GameObject|GetGameModeRef))
  ;[1 1 0] Lobby
  (Variables|/Game/Blueprints/GameModes/GameMode_Game.GameMode_Game_C|SetLobbyPlayerNames _gamemoderef LobbyNames)
  (Variables|/Game/Blueprints/GameModes/GameMode_Game.GameMode_Game_C|SetGamePlayerNames _gamemoderef GameNames)
  (Variables|/Game/Blueprints/GameModes/GameMode_Game.GameMode_Game_C|SetLobbyPlayerColors _gamemoderef LobbyColors)
  (Variables|/Game/Blueprints/GameModes/GameMode_Game.GameMode_Game_C|SetGamePlayerColors _gamemoderef GameColors)
  (Variables|/Game/Blueprints/GameModes/GameMode_Game.GameMode_Game_C|SetGameReadyVisible _gamemoderef ReadyVisible)
  (CallFunction|ServerUpdateLobbyforAll))

(event Custom|PickPlayerColor
  (params (AvailableColors :type Array%20of%20Linear%20Color%20Structures))
  ;[0 1 0] Pick player color
  (bind _widgetshown (Utilities|MacCreateWidget true "/Game/Blueprints/Widgets/PlayerColor.PlayerColor_C"))
  (bind _asplayer_color (Utilities|Casting|CastToPlayerColor _widgetshown))
  (bind _output_get (Variables|Widget|SetWidgetPickPlayerColorRef _asplayer_color))
  (Variables|/Game/Blueprints/Widgets/PlayerColor.PlayerColor_C|SetAvailableColors _output_get AvailableColors)
  (Default|ArrangeAvailableColors _output_get self))

(event Custom|StartGameCountDown
  ;[1 1 0] Lobby
  (Default|StartGameStartTimer (Variables|Widget|GetWidgetLobbyRef)))

(event Custom|WaitForPickColor
  ;[1 1 0] Wait for pick
  (bind _widgetshown (Utilities|MacCreateWidget true "/Game/Blueprints/Widgets/Wait.Wait_C"))
  (bind _aswait (Utilities|Casting|CastToWait _widgetshown))
  (bind _output_get (Variables|Widget|SetWidgetWaitRef _aswait))
  (Default|StartWaitforPickColor _output_get self))

(event Custom|ServerRequestRandomName
  (params (Client :type Player%20Controller%20Game%20Object%20Reference))
  ;[0 1 0] Save Username
  (bind _rndusername (Default|GetRandomUsername (Variables|GameObject|GetGameModeRef)))
  (CallFunction|SaveUsername Client _rndusername true))

(event EventEndPlay
  (params (EndPlayReason :type EEndPlayReason%20Enum :default "Destroyed"))
  ;[1 1 0] Add to available colors in case of quit player
  (CallFunction|ServerPlayerQuit))

(fn ConstructionScript)